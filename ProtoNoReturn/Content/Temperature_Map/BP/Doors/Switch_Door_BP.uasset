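; Switch actor that triggers linked doors when the TPS character overlaps it or presses Use in range, optionally requiring a key.
; Overlap either messages DoorsArray directly or enables input; Use checks HasKey when needed, messages the doors and sets linked lights' shutoff probability.
; Keyed switches show a text prompt to keyless players and swap material and light color when LlaveCogida fires.
; The automatic overlap path ignores key possession.
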(event Custom|LlaveCogida
  (if (Variables|Default|GetNeedKey)
    (Rendering|Material|SetMaterial (Variables|Default|GetStaticMesh) 0 "/Game/Temperature_Map/BP/Materials/Switch_On_Mat1.Switch_On_Mat1")
    (Rendering|Components|Light|SetLightColor (Variables|Default|GetPointLight) "(R=0.023159,G=0.000000,B=1.000000,A=1.000000)" true)))

(event Collision|EventActorBeginOverlap
  (params (OtherActor :type Actor%20Object%20Reference))
  (bind _asbp_tps_character (Utilities|Casting|CastToBP_TPS_Character OtherActor))
  (Variables|Default|SetCharacterReference _asbp_tps_character)
  (Variables|Default|SetIsInTrigger true)
  (if (Variables|Default|GetNeedToUse)
    (if (Variables|Default|GetNeedKey)
      (if (Variables|/Game/mContent/mBlueprints/Character/BP_TPS_Character.BP_TPS_Character_C|GetHasKey (Variables|Default|GetCharacterReference))
        _
        (else
          (Rendering|SetVisibility (Variables|Default|GetTexto) true false))))
    (Input|EnableInput (Game|GetPlayerController 0))
    (else
      (for _array_element (Variables|Default|GetDoors_Array)
        (if (Variables|Default|GetNeedKey)
          (if true
            (Class|UsableItemInterface|UseItem(Message) _array_element :!label _label))
          (else
            (goto _label)))))))

(event Collision|EventActorEndOverlap
  (params (OtherActor :type Actor%20Object%20Reference))
  (Utilities|Casting|CastToBP_TPS_Character OtherActor)
  (Variables|Default|SetIsInTrigger false)
  (if (Variables|Default|GetNeedKey)
    (Rendering|SetVisibility (Variables|Default|GetTexto) false false)))

(event EventBeginPlay
  (if (Variables|Default|GetNeedKey)
    (Rendering|Material|SetMaterial (Variables|Default|GetStaticMesh) 0 "/Game/Temperature_Map/BP/Materials/Switch_Off_Mat.Switch_Off_Mat")
    (Rendering|Components|Light|SetLightColor (Variables|Default|GetPointLight) "(R=1.000000,G=0.027873,B=0.000000,A=1.000000)" true)))

(event Input|ActionEvents|InputActionUse
  (params (Key :type Key%20Structure))
  (:Pressed
    (if (Variables|Default|GetIsInTrigger)
      (if (Variables|Default|GetNeedKey)
        (if (Variables|/Game/mContent/mBlueprints/Character/BP_TPS_Character.BP_TPS_Character_C|GetHasKey (Variables|Default|GetCharacterReference))
          (for _array_element (Variables|Default|GetDoors_Array) :!label _label
            (Class|UsableItemInterface|UseItem(Message) _array_element))
          (for _array_element_2 (Variables|Default|GetLights)
            (Variables|/Game/Diseño/Luz.Luz_C|SetprobabilidadApagar _array_element_2 0.1)))
        (else
          (goto _label))))))

(fn ConstructionScript)