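; BP_Shotgun is the shotgun weapon Blueprint, providing a laser sight while the player aims.
; Each Tick while aiming, it shows the LaserBeam, reapplies its particle template and line-traces forward on the Camera channel, ending the beam at the hit or maximum range.
; When not aiming, it collapses the beam by setting both endpoints to the start point rather than hiding it.
; The construction script makes the Shotgun component ignore all collision channels.
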(event EventTick
  (params (DeltaSeconds :type Float%20%28single-precision%29))
  (if (Variables|Default|GetPlayerIsAiming)
    (Rendering|SetVisibility (Variables|Default|GetLaserBeam) true false)
    (CallFunction|Laser)
    (bind (_start_vector _end_vector) (CallFunction|MForwardVectorComponent (Variables|Default|GetLaserBeam) 5e+03))
    (bind (_outhit _returnvalue) (Collision|LineTraceByChannel _start_vector _end_vector "TraceTypeQuery2" false 0 "None"))
    (if _returnvalue
      (Variables|Default|SetLaserTarget (.Location (Collision|BreakHitResult _outhit)))
      (else
        (Variables|Default|SetLaserTarget _end_vector)))
    (Class|ParticleSystemComponent|SetBeamSourcePoint (Variables|Default|GetLaserBeam) 0 _start_vector)
    (Class|ParticleSystemComponent|SetBeamTargetPoint (Variables|Default|GetLaserBeam) 0 (Variables|Default|GetLaserTarget))
    (else
      (bind _start_vector_2 (CallFunction|MForwardVectorComponent (Variables|Default|GetLaserBeam) 5e+03))
      (Class|ParticleSystemComponent|SetBeamSourcePoint (Variables|Default|GetLaserBeam) 0 _start_vector_2)
      (Class|ParticleSystemComponent|SetBeamTargetPoint (Variables|Default|GetLaserBeam) 0 _start_vector_2))))

(fn ConstructionScript
  (Collision|SetCollisionResponsetoAllChannels (Variables|Default|GetShotgun) "ECR_Ignore"))

(fn Laser
  (Effects|Components|ParticleSystem|SetTemplate (Variables|Default|GetLaserBeam) "/Game/Khiontent/Particles/LaserPS.LaserPS"))