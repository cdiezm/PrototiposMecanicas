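; Trigger actor that fades a configurable on-screen text message in and back out when the TPS character overlaps it.
; BeginPlay creates a W_PrintMessage widget with the set text and color, and overlap starts a timer counting up.
; Tick sets widget opacity from that timer, which overshoots the fade-in time by half the hold time before counting down, producing a full-opacity hold.
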(event EventBeginPlay
  (bind _messagecolor (Variables|Default|GetMessageColor))
  (bind (_r _g _b) (Utilities|Struct|BreakLinearColor _messagecolor))
  (bind _returnvalue (UserInterface|CreateWidget "/Game/Khiontent/Widgets/W_PrintMessage.W_PrintMessage_C"))
  (bind _output_get (Variables|Default|SetMessageWidget _returnvalue))
  (UserInterface|Viewport|AddtoViewport _output_get 0)
  (Appearance|SetColorandOpacity (Variables|Default|GetMessageWidget) (Utilities|Struct|MakeLinearColor _r _g _b 0.0) :!class /Script/UMG.UserWidget)
  (Rendering|Components|TextRender|SetText (Variables|/Game/Khiontent/Widgets/W_PrintMessage.W_PrintMessage_C|GetMessageText (Variables|Default|GetMessageWidget)) (Variables|Default|GetMessageText)))

(event Collision|EventActorBeginOverlap
  (params (OtherActor :type Actor%20Object%20Reference))
  (Utilities|Casting|CastToBP_TPS_Character OtherActor)
  (Variables|Default|SetbIsTextAppearing true))

(event EventTick
  (params (DeltaSeconds :type Float%20%28single-precision%29))
  (bind _messagecolor (Variables|Default|GetMessageColor))
  (bind (_r _g _b) (Utilities|Struct|BreakLinearColor _messagecolor))
  (if (Variables|Default|GetbIsTextAppearing)
    (bind _output_get (Variables|Default|SetTimeSinceWidgetIsVisible (+ DeltaSeconds (Variables|Default|GetTimeSinceWidgetIsVisible))))
    (if (< _output_get (+ (Variables|Default|GetTimeForMessageToAppear) (/ (Variables|Default|GetTimeForMessageToKeepShowing) 2.0)))
      _
      (else
        (Variables|Default|SetbIsTextAppearing false)))
    (else
      (bind _output_get_2 (Variables|Default|SetTimeSinceWidgetIsVisible (- (Variables|Default|GetTimeSinceWidgetIsVisible) DeltaSeconds)))
      (if (<= _output_get_2 0.0)
        (Variables|Default|SetTimeSinceWidgetIsVisible 0.0))))
  (Appearance|SetColorandOpacity (Variables|Default|GetMessageWidget) (Utilities|Struct|MakeLinearColor _r _g _b (/ (Variables|Default|GetTimeSinceWidgetIsVisible) (Variables|Default|GetTimeForMessageToAppear))) :!class /Script/UMG.UserWidget))

(fn ConstructionScript)