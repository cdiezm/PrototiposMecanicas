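; BP_CinematicObjective is an actor that can track the Alpha_Level2 enemy's position, apparently as a target for cinematics.
; On BeginPlay it finds all Alpha_Level2 actors and stores the first as EnemyToFollow.
; Each Tick, while that enemy is valid and IsFollowingAlpha is set, it snaps its root component to the enemy's capsule location, without sweep or interpolation.
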(event EventTick
  (params (DeltaSeconds :type Float%20%28single-precision%29))
  (bind _enemytofollow (Variables|Default|GetEnemyToFollow))
  (Utilities|IsValid _enemytofollow
    (:Is%20Valid
      (if (Variables|Default|GetbIsFollowingAlpha)
        (Transformation|SetWorldLocation (Variables|Default|GetDefaultSceneRoot) (Transformation|GetWorldLocation (Variables|/Script/Engine.Character|GetCapsuleComponent _enemytofollow)) false false)))))

(event EventBeginPlay
  (bind _outactors (Actor|GetAllActorsOfClass "/Game/Khiontent/Blueprints/Actors/Alpha_Level2.Alpha_Level2_C"))
  (Variables|Default|SetEnemyToFollow (Utilities|Array|Get(acopy) _outactors)))

(fn ConstructionScript)