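; Third-person player character with aiming, sprinting, a two-shell shotgun, QTE reload, and health that opens the death level at zero.
; TemperatureComp feeds ControlsTemperatureManager, which scales movement speed and adds cold tremor to camera input while aiming.
; Aiming lerps the camera to a spline point, and firing line-traces from the shotgun's sphere components to send damage and spawn decals.
; Tick runs a sphere trace, diffed against the previous set, to toggle interactable highlights.
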(event Custom|ReloadQTEEnded
  (Development|PrintString "QTE ENDED!!")
  (Variables|Default|SetIsInQTE false))

(event EventBeginPlay
  (bind _temperature_comp (Variables|Default|GetTemperature_Comp))
  ;[1 1 1] Set camera position along spline on right click and reset on realease
  (bind _output_get (Variables|Default|SetCameraDefaultPosition (Variables|/Script/Engine.SceneComponent|GetRelativeLocation (Variables|MyCharacter|GetFollowCamera))))
  (Variables|Default|SetCameraTargetPosition _output_get)
  (Variables|/Script/Engine.CharacterMovementComponent|SetMaxWalkSpeed (Variables|Character|GetCharacterMovement) (Variables|Default|GetwalkSpeed))
  ;[1 1 1] DEVELOPMENT Cheats
  (if (Variables|Default|GetbIsAlwaysHot)
    (Variables|/Game/Khiontent/Blueprints/Classes/Temperature_Comp.Temperature_Comp_C|SetMinTemperature _temperature_comp (Variables|/Game/Khiontent/Blueprints/Classes/Temperature_Comp.Temperature_Comp_C|GetMaxTemperature _temperature_comp))))

(event EventThresholdChange
  ;[1 1 1] Cambiar la velocidad de movimiento cuando se cambia de umbral
  (CallFunction|UpdateMovementSpeed))

(event EventTick
  (params (DeltaSeconds :type Float%20%28single-precision%29))
  (bind _followcamera (Variables|MyCharacter|GetFollowCamera))
  (bind _cameratargetposition (Variables|Default|GetCameraTargetPosition))
  (bind _relativelocation (Variables|/Script/Engine.SceneComponent|GetRelativeLocation _followcamera))
  ;[1 1 1] Set camera position along spline on right click and reset on realease
  (if (Variables|Default|Getstartcountdown)
    (Variables|Default|SetElapsedTime (+ (Variables|Default|GetElapsedTime) DeltaSeconds)))
  (if (Math|Vector|NotEqual(Vector) _cameratargetposition _relativelocation 0.01)
    (Transformation|SetRelativeLocation _followcamera (Math|Vector|Lerp(Vector) _cameratargetposition _relativelocation (Variables|Default|GetCameraLerpSpeed)) false false))
  ;[1 1 1] DEVELOPMENT Cheats
  (if (Variables|Default|GetbHasUnlimitedAmmo)
    (Variables|Default|SetLeftBullet true)
    (Variables|Default|SetRightBullet true))
  (|HighlightInteractableItems))

(event EventOnAttack
  (params (Damage :type Float%20%28single-precision%29) (Location :type Vector :default "0, 0, 0"))
  ;[1 1 1] DEVELOPMENT Cheats
  (if (Variables|Default|GetbHasUnlimitedHealth)
    _
    (else
      (Variables|Default|SetcurrentHP (|newHP Damage))))
  ;[1 1 1] Mancha Sangre (Revisar)
  (Default|ManchaSangre (Variables|Default|GetMancha_Sangre))
  ;[1 1 1] Use this for dead effects
  (if (<= (Variables|Default|GetcurrentHP) 0.0)
    (bind _asgame_instance_to_level_muerte (Utilities|Casting|CastToGameInstanceToLevelMuerte (Game|GetGameInstance)))
    (Variables|/Game/Khiontent/Blueprints/GameInstances/GameInstanceToLevelMuerte.GameInstanceToLevelMuerte_C|SetHasDied _asgame_instance_to_level_muerte true)
    (Game|OpenLevel(byName) "MenuMuerte")))

(event Input|ActionEvents|InputActionSprint
  (params (Key :type Key%20Structure))
  ;[1 1 1] Sprint
  (:Pressed
    (if (not (Variables|Default|GetisAiming))
      (Variables|Default|SetisSprinting true)
      (|Reducirmovimientocamara)
      (CallFunction|UpdateMovementSpeed :!label _label)))
  (:Released
    (Variables|Default|SetisSprinting false)
    (|Aumentarmovimientocámara)
    (goto _label)))

(event Input|ActionEvents|InputActionAimButton
  (params (Key :type Key%20Structure))
  ;[1 1 1] Apuntado, cambia velocidad de movimiento y rotación
  (:Pressed
    (if (Variables|Default|GetisSprinting)
      (Variables|Default|SetisSprinting false))
    (CallFunction|PlayerAim true)
    (Variables|Default|SetbUseControllerRotationYaw true))
  (:Released
    (CallFunction|PlayerAim false)
    (Variables|Default|SetbUseControllerRotationYaw false)))

(event Input|ActionEvents|InputActionReload
  (params (Key :type Key%20Structure))
  ;[1 1 1] Disparo y recarga
  (:Pressed
    (if (and (Variables|Default|GetLeftBullet) (Variables|Default|GetRightBullet))
      (Development|PrintString "Tienes el cargador lleno")
      (elif (>= (Variables|Default|GetBulletsInInventory) 1)
        (if (Variables|Default|GetIsInQTE)
          (Default|QTEKeyPressed (Variables|Default|GetQTEComp))
          (else
            (CallFunction|PlayerAim false)
            (Variables|Default|SetIsInQTE true)
            (Default|ReloadStartedComp (Variables|Default|GetQTEComp))))
        (else
          (Development|PrintString "Out of ammo!!!")
          (Audio|PlaySound2D "/Game/Khiontent/Sounds/Gun_Missfire.Gun_Missfire" 0.2))))))

(event Input|ActionEvents|InputActionFire
  (params (Key :type Key%20Structure))
  (bind _array (Utilities|Array|MakeArray "ObjectTypeQuery3" "ObjectTypeQuery1"))
  ;[1 1 1] Disparo y recarga
  (:Pressed
    (if (and (>= (Variables|Default|GetElapsedTime) (Variables|Default|GetShootingTime)) (Variables|Default|GetisAiming))
      (for _array_element (Actor|GetAllChildActors true)
        (Utilities|Casting|CastToBP_Shotgun _array_element)
        (bind (_array_element_2 _array_index) (Utilities|Array|ForEachLoopwithBreak (Actor|GetComponentsByClass _array_element "/Script/Engine.SphereComponent") :!label _label)
          (:LoopBody
            (if (|canShootRightBullet _array_index)
              (Variables|Default|SetRightBullet false)
              (Variables|Default|SetisFiring true)
              (Audio|PlaySound2D "/Game/Extern/StarterContent/Audio/Explosion02.Explosion02")
              (Variables|Default|SetElapsedTime 0.0)
              (bind (_start_vector _end_vector) (CallFunction|MForwardVectorComponent _array_element_2 1.5e+04))
              (bind _outhit (Collision|LineTraceForObjects _start_vector _end_vector _array false 0 "None"))
              (Class|IDamageable|OnAttack(Message) (.HitActor (Collision|BreakHitResult _outhit)) (Variables|Default|Getdamage) (.Location (Collision|BreakHitResult _outhit)))
              (if (== (Utilities|GetClass (.HitActor (Collision|BreakHitResult _outhit))) "/Game/Khiontent/Blueprints/Actors/Alpha.Alpha_C")
                (Development|PrintString "Hello" :!label _label_2)
                (goto _label Break)
                (elif (!= (.HitActor (Collision|BreakHitResult _outhit)) 0)
                  (Game|SpawnActorfromClass "/Game/Khiontent/Blueprints/Actors/PlaneDecalBullet.PlaneDecalBullet_C" (Math|Transform|MakeTransform (.Location (Collision|BreakHitResult _outhit)) (Math|Rotator|MakeRotfromY (.ImpactNormal (Collision|BreakHitResult _outhit))) "0.200000,0.200000,0.200000") "Undefined" 0 0)
                  (goto _label_2)))
              (elif (|canShootLeftBullet _array_index)
                (Variables|Default|SetLeftBullet false)
                (Variables|Default|SetisFiring true)
                (Audio|PlaySound2D "/Game/Extern/StarterContent/Audio/Explosion02.Explosion02")
                (Variables|Default|SetElapsedTime 0.0)
                (bind (_start_vector_2 _end_vector_2) (CallFunction|MForwardVectorComponent _array_element_2 1.5e+04))
                (bind _outhit_2 (Collision|LineTraceForObjects _start_vector_2 _end_vector_2 _array false 0 "None"))
                (Class|IDamageable|OnAttack(Message) (.HitActor (Collision|BreakHitResult _outhit_2)) (Variables|Default|Getdamage) (.Location (Collision|BreakHitResult _outhit_2)))
                (if (== (Utilities|GetClass (.HitActor (Collision|BreakHitResult _outhit_2))) "/Game/Khiontent/Blueprints/Actors/Alpha.Alpha_C")
                  (Development|PrintString "Hello" :!label _label_3)
                  (elif (!= (.HitActor (Collision|BreakHitResult _outhit_2)) 0)
                    (Game|SpawnActorfromClass "/Game/Khiontent/Blueprints/Actors/PlaneDecalBullet.PlaneDecalBullet_C" (Math|Transform|MakeTransform (.Location (Collision|BreakHitResult _outhit_2)) (Math|Rotator|MakeRotfromY (.ImpactNormal (Collision|BreakHitResult _outhit_2))) "0.200000,0.200000,0.200000") "Undefined" 0 0)
                    (goto _label_3)))
                (else
                  (Development|PrintString "Sin Balas!!!!")
                  (Audio|PlaySound2D "/Game/Khiontent/Sounds/Gun_Missfire.Gun_Missfire" 0.2)))))))))
  (:Released
    (Variables|Default|Setstartcountdown true)
    (Utilities|FlowControl|Delay 1.0)
    (Variables|Default|SetisFiring false)))

(event Input|AxisEvents|InputAxisMoveRight
  (params (AxisValue :type Float%20%28single-precision%29))
  ;[1 1 1] Movimiento
  (Pawn|Input|AddMovementInput (Math|Vector|GetRightVector (Math|Rotator|MakeRotator 0.0 0.0 (.Yaw (Math|Rotator|BreakRotator (Pawn|GetControlRotation :!class /Script/Engine.Pawn))))) AxisValue false)
  (CallFunction|SetHorizontalRotation (< AxisValue -0.1) (> AxisValue 0.1)))

(event Input|AxisEvents|InputAxisMoveForward
  (params (AxisValue :type Float%20%28single-precision%29))
  ;[1 1 1] Movimiento
  (Pawn|Input|AddMovementInput (Math|Vector|GetForwardVector (Math|Rotator|MakeRotator 0.0 0.0 (.Yaw (Math|Rotator|BreakRotator (Pawn|GetControlRotation :!class /Script/Engine.Pawn))))) AxisValue false)
  (CallFunction|SetHorizontalRotation (< AxisValue -0.1) (> AxisValue 0.1)))

(event Input|AxisEvents|InputAxisLookUp
  (params (AxisValue :type Float%20%28single-precision%29))
  (bind _temperature_comp (Variables|Default|GetTemperature_Comp))
  ;[1 1 1] Modify values with cold
  (bind _output_get (Variables|Default|SetTemporaryYaw AxisValue))
  ;;[1 1 1] Para que al no apuntar la cámara no vaya lenta, unir True con el nodo blanco (y abajo)
  (if (not (Variables|Default|GetisAiming))
    _
    (else
      (bind (_rotationafternoise _currenttremornoise) (Default|ApplyCold (Variables|Default|GetControlsTemperatureManager) _output_get (Variables|/Game/Khiontent/Blueprints/Classes/Temperature_Comp.Temperature_Comp_C|GetTemperature _temperature_comp) (Variables|/Game/Khiontent/Blueprints/Classes/Temperature_Comp.Temperature_Comp_C|GetMaxTemperature _temperature_comp) (Variables|/Game/Khiontent/Blueprints/Classes/Temperature_Comp.Temperature_Comp_C|GetMinTemperature _temperature_comp) (Variables|/Game/Khiontent/Blueprints/Classes/Temperature_Comp.Temperature_Comp_C|GetHotterThreshold _temperature_comp) (Variables|/Game/Khiontent/Blueprints/Classes/Temperature_Comp.Temperature_Comp_C|GetColderThreshold _temperature_comp) (Variables|Default|GetCurrentYawDeviation) (Variables|Default|GetisAiming) true))
      (Variables|Default|SetTemporaryYaw _rotationafternoise)
      (Variables|Default|SetCurrentYawDeviation _currenttremornoise)))
  ;[1 1 1] Camera Movement Inputs
  (Pawn|Input|AddControllerPitchInput (* (Variables|Default|GetTemporaryYaw) (Variables|Default|GetBaseTurnRate) (Utilities|Time|GetWorldDeltaSeconds)))
  (bind _outactors (Actor|GetAllActorsOfClass "/Game/Khiontent/Blueprints/Actors/BP_Shotgun.BP_Shotgun_C"))
  ;[1 1 1] Movimiento linterna
  (for _array_element _outactors
    (if (not (Variables|Default|GetisAiming))
      _)))

(event Input|AxisEvents|InputAxisTurn
  (params (AxisValue :type Float%20%28single-precision%29))
  (bind _temperature_comp (Variables|Default|GetTemperature_Comp))
  ;[1 1 1] Modify values with cold
  (bind _output_get (Variables|Default|SetTemporaryPitch AxisValue))
  (if (not (Variables|Default|GetisAiming))
    _
    (else
      (bind (_rotationafternoise _currenttremornoise) (Default|ApplyCold (Variables|Default|GetControlsTemperatureManager) _output_get (Variables|/Game/Khiontent/Blueprints/Classes/Temperature_Comp.Temperature_Comp_C|GetTemperature _temperature_comp) (Variables|/Game/Khiontent/Blueprints/Classes/Temperature_Comp.Temperature_Comp_C|GetMaxTemperature _temperature_comp) (Variables|/Game/Khiontent/Blueprints/Classes/Temperature_Comp.Temperature_Comp_C|GetMinTemperature _temperature_comp) (Variables|/Game/Khiontent/Blueprints/Classes/Temperature_Comp.Temperature_Comp_C|GetHotterThreshold _temperature_comp) (Variables|/Game/Khiontent/Blueprints/Classes/Temperature_Comp.Temperature_Comp_C|GetColderThreshold _temperature_comp) (Variables|Default|GetCurrentPitchDeviation) (Variables|Default|GetisAiming) true))
      (Variables|Default|SetTemporaryPitch _rotationafternoise)
      (Variables|Default|SetCurrentPitchDeviation _currenttremornoise)))
  ;[1 1 1] Camera Movement Inputs
  (Pawn|Input|AddControllerYawInput (* (Variables|Default|GetTemporaryPitch) (Variables|Default|GetBaseLookUpRate) (Utilities|Time|GetWorldDeltaSeconds)))
  (bind _outactors (Actor|GetAllActorsOfClass "/Game/Khiontent/Blueprints/Actors/BP_Shotgun.BP_Shotgun_C"))
  ;[1 1 1] Movimiento linterna
  (for _array_element _outactors
    (if (not (Variables|Default|GetisAiming))
      _)))

(fn ConstructionScript
  (bind _returnvalue (AddComponent|AddChildActorComponent false (Math|Transform|MakeTransform "0, 0, 0")))
  (Transformation|AttachComponentToComponent _returnvalue (Variables|Character|GetMesh) "shotgun_weapon" "KeepRelative" "KeepRelative" "KeepRelative" true))

(fn Base0360To+-180
  (params (ControlerIn :type Float%20%28single-precision%29))
  (return (- ControlerIn 3.6e+02)))

(fn UpdateMovementSpeed
  (bind _charactermovement (Variables|Character|GetCharacterMovement))
  (if (Variables|Default|GetisAiming)
    (bind _valueaftercold (CallFunction|ScaleSpeedwithCold (Variables|Default|GetaimSpeed)))
    (Variables|/Script/Engine.CharacterMovementComponent|SetMaxWalkSpeed (Variables|Character|GetCharacterMovement) _valueaftercold)
    (elif (Variables|Default|GetisSprinting)
      (bind _valueaftercold_2 (CallFunction|ScaleSpeedwithCold (Variables|Default|GetsprintSpeed)))
      (Variables|/Script/Engine.CharacterMovementComponent|SetMaxWalkSpeed _charactermovement _valueaftercold_2)
      (else
        (bind _valueaftercold_3 (CallFunction|ScaleSpeedwithCold (Variables|Default|GetwalkSpeed)))
        (Variables|/Script/Engine.CharacterMovementComponent|SetMaxWalkSpeed _charactermovement _valueaftercold_3)))))

(fn SetHorizontalRotation
  (params (A :type Boolean) (B :type Boolean))
  (bind _returnvalue (Transformation|GetActorRotation))
  (bind _returnvalue_2 (Pawn|GetControlRotation :!class /Script/Engine.Pawn))
  (bind _returnvalue_3 (Transformation|GetActorRotation))
  (if (or A B)
    (if (> (.yaw _returnvalue_2) 1.8e+02)
      (bind _controllerout (CallFunction|Base0360To+-180 (.yaw _returnvalue_2)))
      (if (|ActorOutRanged (.yaw _returnvalue_3) _controllerout)
        (Transformation|SetActorRotation (Math|Rotator|MakeRotator (.roll _returnvalue_3) (.pitch _returnvalue_3) _controllerout))
        (else
          (Transformation|SetActorRotation (Math|Rotator|MakeRotator (.roll _returnvalue_3) (.pitch _returnvalue_3) (Math|Float|Lerp (.yaw _returnvalue_3) _controllerout (Variables|Default|GetlerpValue))))))
      (elif (< (.yaw _returnvalue_3) 0.0)
        (Transformation|SetActorRotation (Math|Rotator|MakeRotator (.roll _returnvalue) (.pitch _returnvalue) (.yaw _returnvalue_2)))
        (else
          (Transformation|SetActorRotation (Math|Rotator|MakeRotator (.roll _returnvalue) (.pitch _returnvalue) (Math|Float|Lerp (.yaw _returnvalue) (.yaw _returnvalue_2) (Variables|Default|GetlerpValue)))))))))

(fn SetVerticalRotation
  (params (A :type Boolean) (b :type Boolean))
  (bind _returnvalue (Transformation|GetActorRotation))
  (bind _returnvalue_2 (Pawn|GetControlRotation :!class /Script/Engine.Pawn))
  (bind _returnvalue_3 (Transformation|GetActorRotation))
  (if (or A b)
    (if (> (.pitch _returnvalue_2) 1.8e+02)
      (bind _controllerout (CallFunction|Base0360To+-180 (.pitch _returnvalue_2)))
      (if (|ActorOutRanged_2 (.pitch _returnvalue_3) _controllerout)
        (Transformation|SetActorRotation (Math|Rotator|MakeRotator (.roll _returnvalue_3) _controllerout (.yaw _returnvalue_3)))
        (else
          (Transformation|SetActorRotation (Math|Rotator|MakeRotator (.roll _returnvalue_3) (Math|Float|Lerp (.pitch _returnvalue_3) _controllerout (Variables|Default|GetlerpValue)) (.yaw _returnvalue_3)))))
      (elif (< (.pitch _returnvalue_3) 0.0)
        (Transformation|SetActorRotation (Math|Rotator|MakeRotator (.roll _returnvalue) (.pitch _returnvalue_2) (.yaw _returnvalue)))
        (else
          (Transformation|SetActorRotation (Math|Rotator|MakeRotator (.roll _returnvalue) (Math|Float|Lerp (.pitch _returnvalue) (.pitch _returnvalue_2) (Variables|Default|GetlerpValue)) (.yaw _returnvalue))))))))

(fn ScaleSpeedwithCold
  (params (Value :type Float%20%28single-precision%29))
  (bind _temperature_comp (Variables|Default|GetTemperature_Comp))
  (bind _valueaftercold (Default|ScalewithCold (Variables|Default|GetControlsTemperatureManager) Value (Variables|/Game/Khiontent/Blueprints/Classes/Temperature_Comp.Temperature_Comp_C|GetTemperature _temperature_comp) (Variables|/Game/Khiontent/Blueprints/Classes/Temperature_Comp.Temperature_Comp_C|GetMaxTemperature _temperature_comp) (Variables|/Game/Khiontent/Blueprints/Classes/Temperature_Comp.Temperature_Comp_C|GetMinTemperature _temperature_comp) (Variables|/Game/Khiontent/Blueprints/Classes/Temperature_Comp.Temperature_Comp_C|GetHotterThreshold _temperature_comp) (Variables|/Game/Khiontent/Blueprints/Classes/Temperature_Comp.Temperature_Comp_C|GetColderThreshold _temperature_comp) false))
  (return _valueaftercold))

(fn PlayerAim
  (params (Start :type Boolean))
  (if Start
    (if (not (Variables|Default|GetIsInQTE))
      (Variables|Default|SetisAiming true)
      (CallFunction|UpdateMovementSpeed)
      (Variables|Default|SetCameraTargetPosition (Spline|GetLocationatSplinePoint (Variables|Default|GetSpline) 1 "Local"))
      (Variables|Default|SetIsAiming true)
      (bind _outactors (Actor|GetAllActorsOfClass "/Game/Khiontent/Blueprints/Actors/BP_Shotgun.BP_Shotgun_C"))
      (for _array_element _outactors
        (Variables|/Game/Khiontent/Blueprints/Actors/BP_Shotgun.BP_Shotgun_C|SetPlayerIsAiming _array_element true)))
    (else
      (Variables|Default|SetisAiming false)
      (if (not (Variables|Default|GetIsInQTE))
        (CallFunction|UpdateMovementSpeed)
        (Variables|Default|SetCameraTargetPosition (Variables|Default|GetCameraDefaultPosition))
        (Variables|Default|SetIsAiming false)
        (bind _outactors_2 (Actor|GetAllActorsOfClass "/Game/Khiontent/Blueprints/Actors/BP_Shotgun.BP_Shotgun_C"))
        (for _array_element_2 _outactors_2
          (Variables|/Game/Khiontent/Blueprints/Actors/BP_Shotgun.BP_Shotgun_C|SetPlayerIsAiming _array_element_2 false))))))