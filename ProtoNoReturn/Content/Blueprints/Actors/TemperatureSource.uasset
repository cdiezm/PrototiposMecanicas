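; Temperature source actor that applies heat or cold to TPS characters within a configurable sphere radius.
; Begin and end overlap events maintain a list of the characters' temperature components.
; Each tick it scales the source temperature linearly by horizontal distance, clamps negative results to zero and appends the value to each component's external temperature list.
; The falloff function also prints debug values.
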(event EventBeginPlay)

(event Collision|EventActorBeginOverlap
  (params (OtherActor :type Actor%20Object%20Reference))
  (bind _asbp_tps_character (Utilities|Casting|CastToBP_TPS_Character OtherActor))
  (Utilities|Array|Add (Variables|Default|GetTemperatureCompList) (Actor|GetComponentbyClass _asbp_tps_character "/Game/Blueprints/Classes/Temperature_Comp.Temperature_Comp_C")))

(event EventTick
  (params (DeltaSeconds :type Float%20%28single-precision%29))
  (for _array_element (Variables|Default|GetTemperatureCompList)
    (bind _tempbydistance (CallFunction|GetTempbyDistance (Transformation|GetHorizontalDistanceTo (Components|GetOwner _array_element)) (Variables|/Script/Engine.SphereComponent|GetSphereRadius (Variables|Default|GetSphere)) (Variables|Default|GetTemperature)))
    (Utilities|Array|Add (Variables|/Game/Blueprints/Classes/Temperature_Comp.Temperature_Comp_C|GetExternTempList _array_element) _tempbydistance)))

(event Collision|EventActorEndOverlap
  (params (OtherActor :type Actor%20Object%20Reference))
  (bind _asbp_tps_character (Utilities|Casting|CastToBP_TPS_Character OtherActor))
  (Utilities|Array|RemoveItem (Variables|Default|GetTemperatureCompList) (Actor|GetComponentbyClass _asbp_tps_character "/Game/Blueprints/Classes/Temperature_Comp.Temperature_Comp_C")))

(fn ConstructionScript
  (Components|Sphere|SetSphereRadius (Variables|Default|GetSphere) (Variables|Default|GetSphereRad) true))

(fn GetTempbyDistance
  (params (ActorDistance :type Float%20%28single-precision%29) (SphereRadius :type Float%20%28single-precision%29) (SourceTemp :type Float%20%28single-precision%29))
  (Development|PrintString (Utilities|String|Append "" "Actor distance: " (Utilities|String|ToString(Float) ActorDistance)) true true "(R=0.000000,G=0.660000,B=1.000000,A=1.000000)" 0.0)
  (LocalVariables|SetAux (* (/ (- SphereRadius ActorDistance) SphereRadius) SourceTemp))
  (if (< (LocalVariables|GetAux) 0.0)
    (LocalVariables|SetAux 0.0))
  (Development|PrintString (Utilities|String|Append "Temperature by distance: " (Utilities|String|ToString(Float) (LocalVariables|GetAux))) true true "(R=0.000000,G=0.660000,B=1.000000,A=1.000000)" 0.0)
  (return (LocalVariables|GetAux)))