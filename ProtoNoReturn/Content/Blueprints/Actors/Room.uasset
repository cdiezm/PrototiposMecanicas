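; Room actor that defines an ambient temperature for the TPS character's temperature component.
; On BeginPlay it writes RoomTemperature to CurrentRoomTemp on the first character found in the level, and again to any such character that begins overlapping it.
; A separate GetCurrentTemperature function adds the room's temperature and all TemperatureSources to CurrentTemperature, but neither event uses it.
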(event EventBeginPlay
  (bind _outactors (Actor|GetAllActorsOfClass "/Game/mContent/mBlueprints/Character/BP_TPS_Character.BP_TPS_Character_C"))
  (Variables|/Game/Blueprints/Classes/Temperature_Comp.Temperature_Comp_C|SetCurrentRoomTemp (Actor|GetComponentbyClass (Utilities|Array|Get(acopy) _outactors) "/Game/Blueprints/Classes/Temperature_Comp.Temperature_Comp_C") (Variables|Default|GetRoomTemperature)))

(event Collision|EventActorBeginOverlap
  (params (OtherActor :type Actor%20Object%20Reference))
  (bind _asbp_tps_character (Utilities|Casting|CastToBP_TPS_Character OtherActor))
  (Variables|/Game/Blueprints/Classes/Temperature_Comp.Temperature_Comp_C|SetCurrentRoomTemp (Actor|GetComponentbyClass _asbp_tps_character "/Game/Blueprints/Classes/Temperature_Comp.Temperature_Comp_C") (Variables|Default|GetRoomTemperature)))

(event EventTick
  (params (DeltaSeconds :type Float%20%28single-precision%29)))

(fn ConstructionScript)

(fn GetCurrentTemperature
  (for _array_element (Variables|Default|GetTemperatureSources)
    (Variables|Default|SetCurrentTemperature (+ (Variables|/Game/Blueprints/Actors/TemperatureSource.TemperatureSource_C|GetTemperature _array_element) (Variables|Default|GetCurrentTemperature))))
  (bind _output_get (Variables|Default|SetCurrentTemperature (+ (Variables|Default|GetRoomTemperature) (Variables|Default|GetCurrentTemperature))))
  (return _output_get))