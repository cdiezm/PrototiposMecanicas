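; Door switch actor that sends UseItemMessage to its linked doors, either on player overlap or on Use input inside its trigger.
; NeedToUse selects the mode; NeedKey makes Use require the character's HasKey, though overlap mode skips that check.
; Timelines fade the point light's intensity with color showing switch state, and a text prompt appears when the key is missing.
; Successful use also sets ProbabilidadApagar on linked Lights.
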(event Custom|LlaveCogida
  (if (Variables|Default|GetNeedKey)
    _))

(event Collision|EventActorBeginOverlap
  (params (OtherActor :type Actor%20Object%20Reference))
  (bind _asbp_tps_character (Utilities|Casting|CastToBP_TPS_Character OtherActor))
  (Variables|Default|SetCharacterReference _asbp_tps_character)
  (Variables|Default|SetIsInTrigger true)
  (if (Variables|Default|GetNeedToUse)
    (if (Variables|Default|GetNeedKey)
      (if (Variables|/Game/mContent/mBlueprints/Character/BP_TPS_Character.BP_TPS_Character_C|GetHasKey (Variables|Default|GetCharacterReference))
        (Input|EnableInput (Game|GetPlayerController 0))
        (bind _alpha (Timeline|Timeline_3 PlayFromStart)
          (:Update
            (Rendering|Components|Light|SetIntensity (Variables|Default|GetPointLight) (Math|Float|Lerp (Variables|Default|GetLightMinimunIntensity) (Variables|Default|GetLightFullIntensity) _alpha))
            (Rendering|Components|Light|SetLightColor (Variables|Default|GetPointLight) (Variables|Default|GetIsInTriggerKeyNeededColor) true))
          (:Finished
            (Input|EnableInput (Game|GetPlayerController 0))))
        (else
          (Rendering|SetVisibility (Variables|Default|GetTexto) true false)
          (Timeline|Timeline_3 PlayFromStart)))
      (else
        (Input|EnableInput (Game|GetPlayerController 0))
        (bind _alpha_2 (Timeline|Timeline_0 Play)
          (:Update
            (Rendering|Components|Light|SetIntensity (Variables|Default|GetPointLight) (Math|Float|Lerp (Variables|Default|GetLightMinimunIntensity) (Variables|Default|GetLightFullIntensity) _alpha_2))
            (Rendering|Components|Light|SetLightColor (Variables|Default|GetPointLight) (Variables|Default|GetIsInTriggerBaseColor) true)))))
    (else
      (for _array_element (Variables|Default|GetDoors_Array)
        (if (Variables|Default|GetNeedKey)
          (if true
            (Class|UsableItemInterface|UseItem(Message) _array_element :!label _label))
          (else
            (goto _label)))))))

(event Collision|EventActorEndOverlap
  (params (OtherActor :type Actor%20Object%20Reference))
  (Utilities|Casting|CastToBP_TPS_Character OtherActor)
  (Variables|Default|SetIsInTrigger false)
  (if (Variables|Default|GetNeedKey)
    (Rendering|SetVisibility (Variables|Default|GetTexto) false false)
    (bind _alpha (Timeline|Timeline_2 ReverseFromEnd)
      (:Update
        (Rendering|Components|Light|SetIntensity (Variables|Default|GetPointLight) (Math|Float|Lerp (Variables|Default|GetLightMinimunIntensity) (Variables|Default|GetLightFullIntensity) _alpha))
        (Rendering|Components|Light|SetLightColor (Variables|Default|GetPointLight) (Variables|Default|GetKeyNeededColor) true)))
    (else
      (bind _alpha_2 (Timeline|Timeline_1 ReverseFromEnd)
        (:Update
          (Rendering|Components|Light|SetIntensity (Variables|Default|GetPointLight) (Math|Float|Lerp (Variables|Default|GetLightMinimunIntensity) (Variables|Default|GetLightFullIntensity) _alpha_2)))
        (:Finished
          (Rendering|Components|Light|SetLightColor (Variables|Default|GetPointLight) (Variables|Default|GetBaseColor) true))))))

(event EventBeginPlay
  (if (Variables|Default|GetNeedKey)
    (Rendering|Components|Light|SetIntensity (Variables|Default|GetPointLight) (Variables|Default|GetLightMinimunIntensity))
    (Rendering|Components|Light|SetLightColor (Variables|Default|GetPointLight) (Variables|Default|GetKeyNeededColor) true)
    (else
      (Rendering|Components|Light|SetIntensity (Variables|Default|GetPointLight) (Variables|Default|GetLightMinimunIntensity))
      (Rendering|Components|Light|SetLightColor (Variables|Default|GetPointLight) (Variables|Default|GetBaseColor) true))))

(event Input|ActionEvents|InputActionUse
  (params (Key :type Key%20Structure))
  (:Pressed
    (if (Variables|Default|GetIsInTrigger)
      (if (Variables|Default|GetNeedKey)
        (if (Variables|/Game/mContent/mBlueprints/Character/BP_TPS_Character.BP_TPS_Character_C|GetHasKey (Variables|Default|GetCharacterReference))
          (for _array_element (Variables|Default|GetDoors_Array) :!label _label
            (Class|UsableItemInterface|UseItem(Message) _array_element))
          (for _array_element_2 (Variables|Default|GetLights)
            (Variables|/Game/Diseño/Luz.Luz_C|SetprobabilidadApagar _array_element_2 0.1)))
        (else
          (goto _label))))))

(fn ConstructionScript)