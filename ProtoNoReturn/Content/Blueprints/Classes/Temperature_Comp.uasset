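; Temperature component that tracks a body temperature drifting toward its surroundings, clamped between minimum and maximum limits.
; Each Tick moves Temperature toward the external value at a rate slowed by ColdProtection, then prints debug readouts.
; The external value is the room temperature plus all ExternTempList entries, a sum despite the GetAverageTemp name.
; The list clears every Tick, so sources only count for the frame they are added.
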(event EventTick
  (params (DeltaSeconds :type Float%20%28single-precision%29))
  (bind _externtemp (CallFunction|GetAverageTemp (Variables|Default|GetExternTempList) (Variables|Default|GetCurrentRoomTemp)))
  (Variables|Default|SetExternTemperature _externtemp)
  (Variables|Default|SetTemperature (Math|Float|Clamp(Float) (+ (* (* DeltaSeconds (/ (- (Variables|Default|GetTemperature) (Variables|Default|GetExternTemperature)) (Variables|Default|GetColdProtection))) -1.0) (Variables|Default|GetTemperature)) (Variables|Default|GetMinTemperature) (Variables|Default|GetMaxTemperature)))
  (Development|PrintString (Utilities|String|Append "Temperature: " (Utilities|String|ToString(Float) (Variables|Default|GetTemperature))) true true "(R=0.000000,G=0.660000,B=1.000000,A=1.000000)" 0.0)
  (Development|PrintString (Utilities|String|Append "Room Temp: " (Utilities|String|ToString(Float) (Variables|Default|GetCurrentRoomTemp))) true true "(R=0.000000,G=0.660000,B=1.000000,A=1.000000)" 0.0)
  (Development|PrintString (Utilities|String|Append "Extern Temperature: " (Utilities|String|ToString(Float) (Variables|Default|GetExternTemperature))) true true "(R=0.000000,G=0.660000,B=1.000000,A=1.000000)" 0.0)
  (Utilities|Array|Clear (Variables|Default|GetExternTempList)))

(fn GetCurrentTemperature
  (params (CurrentRoom :type Room%20Object%20Reference))
  (bind _currenttemperature (Default|GetCurrentTemperature CurrentRoom))
  (return _currenttemperature))

(fn GetAverageTemp
  (params (ExternTempList :type Array%20of%20Floats%20%28single-precision%29) (RoomTemp :type Float%20%28single-precision%29))
  (if (<= (Utilities|Array|Length ExternTempList) 0)
    (return RoomTemp)
    (else
      (for _array_element ExternTempList
        (LocalVariables|SetTotal (+ (LocalVariables|GetTotal) _array_element)))
      (bind _output_get (LocalVariables|SetTotal (+ RoomTemp (LocalVariables|GetTotal))))
      (return _output_get))))