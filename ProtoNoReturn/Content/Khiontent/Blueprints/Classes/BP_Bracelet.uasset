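; BP_Bracelet is the bracelet energy model powering the flashlight, thermal vision and heating.
; Each Tick it subtracts standby and active-feature drain, adds recharge and clamps energy to its maximum.
; Two mutually resetting DoOnce nodes notify the owner once per crossing of the ten percent threshold.
; Functions toggle features, adjust recharge additively, and copy settings and state to another bracelet, except thermal vision state.
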(event EventBeginPlay
  (Variables|Default|SetCurrentEnergy (Variables|Default|GetInitialEnergy)))

(event EventTick
  (params (DeltaSeconds :type Float%20%28single-precision%29))
  (Variables|Default|SetCurrentEnergy (Math|Float|Clamp(Float) (+ (- (- (- (- (Variables|Default|GetCurrentEnergy) (* DeltaSeconds (Variables|Default|GetEnergyLostPerSecondOnStandby))) (* DeltaSeconds (Variables|Default|GetEnergyConsumedPerSecondByFlashlight) (Math|Conversions|ToFloat(Boolean) (Variables|Default|GetbIsFlashlightActive)))) (* (Variables|Default|GetEnergyConsumedPerSecondByThermalVision) (Math|Conversions|ToFloat(Boolean) (Variables|Default|GetbIsThermalVisionActive)) DeltaSeconds)) (* (Variables|Default|GetEnergyConsumedPerSecondByHeating) (Math|Conversions|ToFloat(Boolean) (Variables|Default|GetbIsHeatingActive)) DeltaSeconds)) (* (Variables|Default|GetEnergyGainedPerSecond) DeltaSeconds)) 0.0 (Variables|Default|GetMaxEnergy)))
  (bind _outenergypercentage (CallFunction|GetCurrentEnergyPercentage))
  (if (>= _outenergypercentage 0.1)
    (Utilities|FlowControl|DoOnce false :!label _label
      (:Completed
        (Class|BPBraceletOwnerInterface|ChangeBraceletThreshold(Message) (Components|GetOwner))
        (goto _label_2 Reset)))
    (else
      (Utilities|FlowControl|DoOnce false :!label _label_2
        (:Completed
          (Class|BPBraceletOwnerInterface|ChangeBraceletThreshold(Message) (Components|GetOwner) 1)
          (goto _label Reset))))))

(fn ChangeRechargeRate
  (params (InEnergyGainedPerSecond :type Float%20%28single-precision%29))
  (Variables|Default|SetEnergyGainedPerSecond (+ InEnergyGainedPerSecond (Variables|Default|GetEnergyGainedPerSecond)))
  (return))

(fn ChangeThermalVisionState
  (params (bInIsThermalVisionActivated :type Boolean))
  (Variables|Default|SetbIsThermalVisionActive bInIsThermalVisionActivated)
  (return))

(fn TransferValuestoAnotherBracelet
  (params (DestinationBracelet :type BP%20Bracelet%20Object%20Reference))
  (Variables|BP_Bracelet_C|SetInitialEnergy DestinationBracelet (Variables|Default|GetInitialEnergy))
  (Variables|BP_Bracelet_C|SetMaxEnergy DestinationBracelet (Variables|Default|GetMaxEnergy))
  (Variables|BP_Bracelet_C|SetEnergyLostPerSecondOnStandby DestinationBracelet (Variables|Default|GetEnergyLostPerSecondOnStandby))
  (Variables|BP_Bracelet_C|SetEnergyConsumedPerSecondByFlashlight DestinationBracelet (Variables|Default|GetEnergyConsumedPerSecondByFlashlight))
  (Variables|BP_Bracelet_C|SetEnergyConsumedPerSecondByThermalVision DestinationBracelet (Variables|Default|GetEnergyConsumedPerSecondByThermalVision))
  (Variables|BP_Bracelet_C|SetEnergyConsumedPerSecondByHeating DestinationBracelet (Variables|Default|GetEnergyConsumedPerSecondByHeating))
  (Variables|BP_Bracelet_C|SetCurrentEnergy DestinationBracelet (Variables|Default|GetCurrentEnergy))
  (Variables|BP_Bracelet_C|SetbIsFlashlightActive DestinationBracelet (Variables|Default|GetbIsFlashlightActive))
  (Variables|BP_Bracelet_C|SetbIsHeatingActive DestinationBracelet (Variables|Default|GetbIsHeatingActive))
  (Variables|BP_Bracelet_C|SetEnergyGainedPerSecond DestinationBracelet (Variables|Default|GetEnergyGainedPerSecond))
  (return))

(fn ChangeFlashlightState
  (params (bInIsFlashlightActive :type Boolean))
  (Variables|Default|SetbIsFlashlightActive bInIsFlashlightActive)
  (return))

(fn ChangeHeatingState
  (params (bInIsHeatingActive :type Boolean))
  (Variables|Default|SetbIsHeatingActive bInIsHeatingActive)
  (return))

(fn GetCurrentEnergyPercentage
  (return (/ (Variables|Default|GetCurrentEnergy) (Variables|Default|GetMaxEnergy))))