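; Component that gives its owning actor a button-mash quick-time event prompt, shown as an on-screen widget.
; On BeginPlay it creates and configures a W_MashQTE widget, then each Tick pins it to the owner's projected screen position.
; The widget is visible only while the character is flagged close and the owner is within the viewport.
; External callers toggle proximity, send taps that count only while visible, query completion and remove the widget.
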(event EventBeginPlay
  (bind _returnvalue (UserInterface|CreateWidget "/Game/Khiontent/Widgets/W_MashQTE.W_MashQTE_C"))
  (bind _output_get (Variables|Default|SetWidgetMashQTE _returnvalue))
  (Default|SetTapColor _output_get (Variables|Default|GetTapColor))
  (Default|SetImage (Variables|Default|GetWidgetMashQTE) (Variables|Default|GetImage))
  (Default|SetTimeUntilColorClears (Variables|Default|GetWidgetMashQTE) (Variables|Default|GetTimeUntilColorClears))
  (Default|SetTotalClearLevel (Variables|Default|GetWidgetMashQTE) (Variables|Default|GetTotalRequired))
  (Default|SetSubtractionPerSecond (Variables|Default|GetWidgetMashQTE) (Variables|Default|GetSubtractionPerSecond))
  (UserInterface|Viewport|AddtoViewport (Variables|Default|GetWidgetMashQTE) 0))

(event EventTick
  (params (DeltaSeconds :type Float%20%28single-precision%29))
  (bind _returnvalue (Components|GetOwner))
  (bind _returnvalue_2 (Viewport|GetViewportSize))
  (bind _returnvalue_3 (Game|GetPlayerController 0))
  (bind _bischaracterclose (Variables|Default|GetbIsCharacterClose))
  (bind _returnvalue_4 (Transformation|GetActorLocation _returnvalue))
  (bind (_x _y) (Math|Vector2D|BreakVector2D _returnvalue_2))
  (bind (_screenlocation _returnvalue_5) (Class|PlayerController|ProjectWorldLocationtoScreen _returnvalue_3 _returnvalue_4 false))
  (bind (_x_2 _y_2) (Math|Vector2D|BreakVector2D _screenlocation))
  (bind _returnvalue_6 (Math|Float|InRange(Float) _x_2 0.0 _x))
  (bind _returnvalue_7 (Math|Float|InRange(Float) _y_2 0.0 _y))
  (bind _returnvalue_8 (Math|Boolean|ANDBoolean _returnvalue_5 _bischaracterclose _returnvalue_6 _returnvalue_7))
  (if _returnvalue_8
    (Default|SetScreenPosition (Variables|Default|GetWidgetMashQTE) _screenlocation))
  (Widget|SetVisibility (Variables|Default|GetWidgetMashQTE) (select _returnvalue_8 "HitTestInvisible" "Hidden")))

(fn Tap
  (switch Utilities|FlowControl|Switch|SwitchonESlateVisibility (Widget|GetVisibility (Variables|Default|GetWidgetMashQTE))
    (:Visible
      _)
    (:HitTestInvisible
      _))
  (Default|Tap (Variables|Default|GetWidgetMashQTE) (Variables|Default|GetAdditionPerTap))
  (return))

(fn ShowWidget
  (Variables|Default|SetbIsCharacterClose true)
  (return))

(fn HideWidget
  (Variables|Default|SetbIsCharacterClose false)
  (return))

(fn IsQTECompleted
  (return (> (Default|GetPercent (Variables|Default|GetWidgetMashQTE)) 0.99)))

(fn DeleteWidget
  (Widget|RemovefromParent (Variables|Default|GetWidgetMashQTE))
  (return))