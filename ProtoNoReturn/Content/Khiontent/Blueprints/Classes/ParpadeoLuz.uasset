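; Actor component for flickering the point or spot light on its owner.
; BeginPlay finds the light, preferring a point light, caches its intensity and starts a looping timer at VelocidadParpadeo intervals.
; Parpadeo randomly sets intensity to zero based on ProbabilidadApagar, otherwise restores the cached value.
; The timer targets "parpadear", which does not match the Parpadeo function shown.
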(event EventBeginPlay
  (bind _returnvalue (Components|GetOwner))
  (bind _returnvalue_2 (Actor|GetComponentbyClass _returnvalue "/Script/Engine.SpotLightComponent"))
  (bind _returnvalue_3 (Actor|GetComponentbyClass _returnvalue "/Script/Engine.PointLightComponent"))
  (Utilities|IsValid _returnvalue_3
    (:Is%20Valid
      (bind _output_get (Variables|Default|SetPointLightComponent _returnvalue_3))
      (Variables|Default|SetEsPointLight true)
      (Variables|Default|SetIntensidadInicial (Variables|/Script/Engine.LightComponentBase|GetIntensity _output_get)))
    (:Is%20Not%20Valid
      (Utilities|IsValid _returnvalue_2
        (:Is%20Valid
          (bind _output_get_2 (Variables|Default|SetSpotLightComponent _returnvalue_2))
          (Variables|Default|SetEsPointLight false)
          (Variables|Default|SetIntensidadInicial (Variables|/Script/Engine.LightComponentBase|GetIntensity _output_get_2))))))
  (Utilities|Time|SetTimerbyFunctionName 0 "parpadear" (Variables|Default|GetvelocidadParpadeo) true))

(fn Parpadeo
  (if (>= (Variables|Default|GetProbabilidadApagar) (Math|Random|RandomFloat))
    (if (Variables|Default|GetEsPointLight)
      (Rendering|Components|Light|SetIntensity (Variables|Default|GetPointLightComponent) 0.0)
      (else
        (Rendering|Components|Light|SetIntensity (Variables|Default|GetSpotLightComponent) 0.0)))
    (elif (Variables|Default|GetEsPointLight)
      (Rendering|Components|Light|SetIntensity (Variables|Default|GetPointLightComponent) (Variables|Default|GetIntensidadInicial))
      (else
        (Rendering|Components|Light|SetIntensity (Variables|Default|GetSpotLightComponent) (Variables|Default|GetIntensidadInicial))))))