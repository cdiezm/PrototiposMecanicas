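; Actor component that runs the reload quick-time event for BP_TPS_Character's left and right bullets.
; It creates the QTEReload widget, passing temperature range and loaded state, and forwards key presses to it.
; The widget's end event loads successful bullets, deducts successes and failures from inventory, then notifies the character.
; With one bullet remaining and both sides empty, it temporarily marks the left loaded.
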(event Custom|ReloadQTEWidgetEnded_Event
  (params (LeftBulletOK :type Boolean) (RightBulletOK :type Boolean) (FailOnLeftBullet :type Boolean) (FailOnRightBullet :type Boolean))
  (bind _asbp_tps_character (Utilities|Casting|CastToBP_TPS_Character (Components|GetOwner)))
  (bind _output_get (Variables|Default|SetPlayer _asbp_tps_character))
  (if (and (Variables|Default|GetIsLastBullet) (and (Variables|/Game/Khiontent/Blueprints/Actors/BP_TPS_Character.BP_TPS_Character_C|GetLeftBullet _output_get) (and (== (Variables|/Game/Khiontent/Blueprints/Actors/BP_TPS_Character.BP_TPS_Character_C|GetBulletsInInventory _output_get) 1) (and (not LeftBulletOK) (not FailOnLeftBullet)))))
    (Variables|/Game/Khiontent/Blueprints/Actors/BP_TPS_Character.BP_TPS_Character_C|SetLeftBullet _output_get false)
    (Variables|Default|SetIsLastBullet false))
  (if LeftBulletOK
    (Variables|/Game/Khiontent/Blueprints/Actors/BP_TPS_Character.BP_TPS_Character_C|SetLeftBullet (Variables|Default|GetPlayer) true)
    (Math|Integer|DecrementInt (Variables|/Game/Khiontent/Blueprints/Actors/BP_TPS_Character.BP_TPS_Character_C|GetBulletsInInventory (Variables|Default|GetPlayer))
      (:%20%20
        _)))
  (if FailOnLeftBullet
    (Math|Integer|DecrementInt (Variables|/Game/Khiontent/Blueprints/Actors/BP_TPS_Character.BP_TPS_Character_C|GetBulletsInInventory (Variables|Default|GetPlayer))
      (:%20%20
        _)))
  (if RightBulletOK
    (Variables|/Game/Khiontent/Blueprints/Actors/BP_TPS_Character.BP_TPS_Character_C|SetRightBullet (Variables|Default|GetPlayer) true)
    (Math|Integer|DecrementInt (Variables|/Game/Khiontent/Blueprints/Actors/BP_TPS_Character.BP_TPS_Character_C|GetBulletsInInventory (Variables|Default|GetPlayer))
      (:%20%20
        _)))
  (if FailOnRightBullet
    (Math|Integer|DecrementInt (Variables|/Game/Khiontent/Blueprints/Actors/BP_TPS_Character.BP_TPS_Character_C|GetBulletsInInventory (Variables|Default|GetPlayer))
      (:%20%20
        _)))
  (Default|ReloadQTEEnded (Variables|Default|GetPlayer)))

(fn ReloadStartedComp
  (bind _returnvalue (Components|GetOwner))
  (bind _returnvalue_2 (Actor|GetComponentbyClass _returnvalue "/Game/Khiontent/Blueprints/Classes/Temperature_Comp.Temperature_Comp_C"))
  (bind _returnvalue_3 (UserInterface|CreateWidget "/Game/Khiontent/Widgets/QTEReload.QTEReload_C"))
  (UserInterface|Viewport|AddtoViewport _returnvalue_3 0)
  (bind _output_get (Variables|Default|SetQTEWidget _returnvalue_3))
  (bind _asbp_tps_character (Utilities|Casting|CastToBP_TPS_Character _returnvalue))
  (if (== (Variables|/Game/Khiontent/Blueprints/Actors/BP_TPS_Character.BP_TPS_Character_C|GetBulletsInInventory _asbp_tps_character) 1)
    (if (and (not (Variables|/Game/Khiontent/Blueprints/Actors/BP_TPS_Character.BP_TPS_Character_C|GetRightBullet _asbp_tps_character)) (not (Variables|/Game/Khiontent/Blueprints/Actors/BP_TPS_Character.BP_TPS_Character_C|GetLeftBullet _asbp_tps_character)))
      (Variables|/Game/Khiontent/Blueprints/Actors/BP_TPS_Character.BP_TPS_Character_C|SetLeftBullet _asbp_tps_character true)
      (Variables|Default|SetIsLastBullet true)))
  (Default|StartQTE _output_get (Variables|/Game/Khiontent/Blueprints/Classes/Temperature_Comp.Temperature_Comp_C|GetTemperature _returnvalue_2) (Variables|/Game/Khiontent/Blueprints/Classes/Temperature_Comp.Temperature_Comp_C|GetMinTemperature _returnvalue_2) (Variables|/Game/Khiontent/Blueprints/Classes/Temperature_Comp.Temperature_Comp_C|GetMaxTemperature _returnvalue_2) (Variables|/Game/Khiontent/Blueprints/Actors/BP_TPS_Character.BP_TPS_Character_C|GetRightBullet _asbp_tps_character) (Variables|/Game/Khiontent/Blueprints/Actors/BP_TPS_Character.BP_TPS_Character_C|GetLeftBullet _asbp_tps_character) self))

(fn QTEKeyPressed
  (Default|PressQTE (Variables|Default|GetQTEWidget)))