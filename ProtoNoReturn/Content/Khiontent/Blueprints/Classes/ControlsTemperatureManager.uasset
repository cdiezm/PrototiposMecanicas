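; Controls temperature manager that alters input values as temperature drops, scaling them and adding hand-tremor noise while aiming.
; Scaling is either continuous or stepped across three threshold bands, with extra multipliers for camera input.
; In stepped mode, band changes notify the owner.
; Tremor is random noise divided by the cold scale, with accumulated offset passed between calls and steered back when it would exceed a maximum radius.
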(event EventBeginPlay)

(event EventTick
  (params (DeltaSeconds :type Float%20%28single-precision%29)))

(fn ScalewithCold
  (params (Value :type Float%20%28single-precision%29) (CurrentTemperature :type Float%20%28single-precision%29) (MaxTemperature :type Float%20%28single-precision%29) (MinTemperature :type Float%20%28single-precision%29) (HigherThreshold :type Float%20%28single-precision%29) (LowerThreshold :type Float%20%28single-precision%29) (bIsCamera :type Boolean))
  (bind _scalecoldthreshold (Variables|Default|GetScaleColdThreshold))
  (bind _scalehotthreshold (Variables|Default|GetScaleHotThreshold))
  (bind _returnvalue (* Value _scalehotthreshold))
  (bind _returnvalue_2 (* Value _scalecoldthreshold))
  (if (Variables|Default|GetbTemperatureDropsContinuously)
    ;[1 1 1] Antigua función sin umbrales
    (return (* Value (Math|Float|MapRangeClamped CurrentTemperature MaxTemperature MinTemperature 1.0 0.1)))
    (elif (> CurrentTemperature HigherThreshold)
      (CallFunction|NotifyifThresholdNotMatching)
      (return Value)
      (elif (<= CurrentTemperature LowerThreshold)
        (CallFunction|NotifyifThresholdNotMatching 2)
        (if bIsCamera
          (return (* (Variables|Default|GetScaleCameraColdThreshold) _returnvalue_2))
          (else
            (return _returnvalue_2)))
        (else
          (CallFunction|NotifyifThresholdNotMatching 1)
          (if bIsCamera
            (return (* (Variables|Default|GetScaleCameraHotThreshold) _returnvalue))
            (else
              (return _returnvalue))))))))

(fn AddRotationNoisewhenCold
  (params (Rotation :type Float%20%28single-precision%29) (CurrentTemperature :type Float%20%28single-precision%29) (MaxTemperature :type Float%20%28single-precision%29) (MinTemperature :type Float%20%28single-precision%29) (HigherThreshold :type Float%20%28single-precision%29) (LowerThreshold :type Float%20%28single-precision%29) (PreviousNoise :type Float%20%28single-precision%29))
  (bind _generatedrandomcoldnumber (LocalVariables|GetGeneratedRandomColdNumber))
  (bind (_bhasbiggerabsolutevalue _addedresult) (|HasBiggerAbsoluteValue PreviousNoise _generatedrandomcoldnumber))
  (|GenerateRandomNumberwithCold CurrentTemperature MaxTemperature MinTemperature HigherThreshold LowerThreshold)
  (if _bhasbiggerabsolutevalue
    (return (- Rotation (LocalVariables|GetGeneratedRandomColdNumber)) (- PreviousNoise (LocalVariables|GetGeneratedRandomColdNumber)))
    (else
      (return (+ Rotation (LocalVariables|GetGeneratedRandomColdNumber)) _addedresult))))

(fn ApplyCold
  (params (Value :type Float%20%28single-precision%29) (CurrentTemperature :type Float%20%28single-precision%29) (MaxTemperature :type Float%20%28single-precision%29) (MinTemperature :type Float%20%28single-precision%29) (HigherThreshold :type Float%20%28single-precision%29) (LowerThreshold :type Float%20%28single-precision%29) (PreviousTremorNoise :type Float%20%28single-precision%29) (bIsAiming :type Boolean) (bIsCamera :type Boolean))
  (bind _output_get (LocalVariables|SetTemporaryValue Value))
  (bind _valueaftercold (CallFunction|ScalewithCold _output_get CurrentTemperature MaxTemperature MinTemperature HigherThreshold LowerThreshold bIsCamera))
  (LocalVariables|SetTemporaryValue _valueaftercold)
  (if (not bIsAiming)
    _
    (else
      (bind (_rotationafternoise _currentnoise) (CallFunction|AddRotationNoisewhenCold (LocalVariables|GetTemporaryValue) CurrentTemperature MaxTemperature MinTemperature HigherThreshold LowerThreshold PreviousTremorNoise))
      (LocalVariables|SetTemporaryValue _rotationafternoise)))
  (return (LocalVariables|GetTemporaryValue) _currentnoise))

(fn NotifyifThresholdNotMatching
  (params (Threshold :type Integer))
  (if (!= (Variables|Default|GetPreviousThreshold) Threshold)
    (Variables|Default|SetPreviousThreshold Threshold)
    (Class|ITemperatureController|ThresholdChange(Message) (Components|GetOwner)))
  (return))