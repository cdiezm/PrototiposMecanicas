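; Player death handler, expected to be owned by BP_TPS_Character, that runs the fade-out and switch to the game-over level.
; DeadFadeOut creates the FadeOutPlayerDead widget, shows it and passes itself to its Init.
; LoadGameOverLevel sets HasDied on GameInstanceToLevelMuerte, false only if the owning character still has HP, then opens MenuMuerte.
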(event Custom|DeadFadeOut
  (bind _returnvalue (UserInterface|CreateWidget "/Game/Khiontent/Widgets/FadeOutPlayerDead.FadeOutPlayerDead_C"))
  (UserInterface|Viewport|AddtoViewport _returnvalue 0)
  (bind _output_get (Variables|Default|SetFadeOutPlayerWidget _returnvalue))
  (Default|Init _output_get self))

(event Custom|LoadGameOverLevel
  (bind _asgame_instance_to_level_muerte (Utilities|Casting|CastToGameInstanceToLevelMuerte (Game|GetGameInstance)))
  (bind _asbp_tps_character (Utilities|Casting|CastToBP_TPS_Character (Components|GetOwner))
    (:then
      (if (> (Variables|/Game/Khiontent/Blueprints/Actors/BP_TPS_Character.BP_TPS_Character_C|GetcurrentHP _asbp_tps_character) 0.0)
        (Variables|/Game/Khiontent/Blueprints/GameInstances/GameInstanceToLevelMuerte.GameInstanceToLevelMuerte_C|SetHasDied _asgame_instance_to_level_muerte false)
        (else
          (Variables|/Game/Khiontent/Blueprints/GameInstances/GameInstanceToLevelMuerte.GameInstanceToLevelMuerte_C|SetHasDied _asgame_instance_to_level_muerte true :!label _label))))
    (:CastFailed
      (goto _label)))
  (Game|OpenLevel(byName) "MenuMuerte"))

(event EventBeginPlay)

(event EventTick
  (params (DeltaSeconds :type Float%20%28single-precision%29)))