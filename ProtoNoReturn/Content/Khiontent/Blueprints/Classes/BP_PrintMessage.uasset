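; BP_PrintMessage is a component that shows a configurable text message on screen, with an optional image beside it.
; BeginPlay creates a W_PrintMessage widget; PrintMessage fills it and starts the display, while StopPrintingMessage zeroes the timer.
; Tick runs one timer up, then down, deriving opacity from it to produce fade-in, hold and fade-out.
; In first-time-only mode, it collapses the widget and destroys itself after showing.
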(event EventBeginPlay
  (bind _messagecolor (Variables|Default|GetMessageColor))
  (bind (_r _g _b) (Utilities|Struct|BreakLinearColor _messagecolor))
  (bind _returnvalue (UserInterface|CreateWidget "/Game/Khiontent/Widgets/W_PrintMessage.W_PrintMessage_C"))
  (bind _output_get (Variables|Default|SetMessageWidget _returnvalue))
  (UserInterface|Viewport|AddtoViewport _output_get 0)
  (Appearance|SetColorandOpacity (Variables|Default|GetMessageWidget) (Utilities|Struct|MakeLinearColor _r _g _b 0.0) :!class /Script/UMG.UserWidget))

(event EventTick
  (params (DeltaSeconds :type Float%20%28single-precision%29))
  (bind _messagecolor (Variables|Default|GetMessageColor))
  (bind (_r _g _b) (Utilities|Struct|BreakLinearColor _messagecolor))
  (if (Variables|Default|GetActivated)
    (if (Variables|Default|GetbIsTextAppearing)
      (bind _output_get (Variables|Default|SetTimeSinceWidgetIsVisible (+ DeltaSeconds (Variables|Default|GetTimeSinceWidgetIsVisible))))
      (if (< _output_get (+ (Variables|Default|GetTimeForMessageToAppear) (/ (Variables|Default|GetTimeForMessageToKeepShowing) 2.0)))
        _
        (else
          (Variables|Default|SetbIsTextAppearing false)))
      (Appearance|SetColorandOpacity (Variables|Default|GetMessageWidget) (Utilities|Struct|MakeLinearColor _r _g _b (/ (Variables|Default|GetTimeSinceWidgetIsVisible) (Variables|Default|GetTimeForMessageToAppear))) :!class /Script/UMG.UserWidget :!label _label)
      (else
        (bind _output_get_2 (Variables|Default|SetTimeSinceWidgetIsVisible (- (Variables|Default|GetTimeSinceWidgetIsVisible) DeltaSeconds)))
        (if (<= _output_get_2 0.0)
          (Variables|Default|SetTimeSinceWidgetIsVisible 0.0)
          (if (Variables|Default|GetbIsActivatedFirstTimeOnly)
            (if (Variables|Default|GetbHasBeenActivated)
              (Widget|SetVisibility (Variables|Default|GetMessageWidget) "Collapsed")
              (Components|DestroyComponent))
            (else
              (goto _label)))
          (else
            (goto _label)))))))

(fn PrintMessage
  (bind _messagecolor (Variables|Default|GetMessageColor))
  (bind _messagewidget (Variables|Default|GetMessageWidget))
  (bind (_r _g _b) (Utilities|Struct|BreakLinearColor _messagecolor))
  (bind _buttonimage (Variables|/Game/Khiontent/Widgets/W_PrintMessage.W_PrintMessage_C|GetButtonImage _messagewidget))
  (if (<= (Variables|Default|GetTimeSinceWidgetIsVisible) 0.0)
    (Variables|Default|SetbIsTextAppearing true :!label _label)
    (Variables|Default|SetbHasBeenActivated true)
    (Appearance|SetColorandOpacity (Variables|Default|GetMessageWidget) (Utilities|Struct|MakeLinearColor _r _g _b (.A (Utilities|Struct|BreakLinearColor (Variables|/Script/UMG.UserWidget|GetColorAndOpacity (Variables|Default|GetMessageWidget))))) :!class /Script/UMG.UserWidget)
    (Rendering|Components|TextRender|SetText (Variables|/Game/Khiontent/Widgets/W_PrintMessage.W_PrintMessage_C|GetMessageText (Variables|Default|GetMessageWidget)) (Variables|Default|GetMessageText))
    (if (not (== (Variables|Default|GetImage) 0))
      (Appearance|SetBrushfromTexture _buttonimage (Variables|Default|GetImage) false)
      (Widget|SetVisibility _buttonimage "Visible")
      (Layout|BorderSlot|SetPadding (Class|WidgetLayoutLibrary|SlotasOverlaySlot (Variables|/Game/Khiontent/Widgets/W_PrintMessage.W_PrintMessage_C|GetMessageText (Variables|Default|GetMessageWidget))) (Utilities|Struct|MakeMargin (Math|Conversions|ToFloat(Integer) (+ (Class|Texture2D|BlueprintGetSizeX (Variables|Default|GetImage)) (Variables|Default|GetSeparationBetweenImageAndText))) 0.0 0.0 0.0) :!class /Script/UMG.OverlaySlot))
    (elif (not (Variables|Default|GetbIsActivatedFirstTimeOnly))
      (goto _label))))

(fn StopPrintingMessage
  (Variables|Default|SetbIsTextAppearing false)
  (Variables|Default|SetTimeSinceWidgetIsVisible 0.0))