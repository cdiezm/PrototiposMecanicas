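; Blueprint function library that toggles highlighting on objects through the Custom Depth render pass.
; StartHighlight clears the old target through StopHighlight, then enables custom depth on the new target's primitive components tagged "Highlight".
; StopHighlight disables custom depth on the same tagged components after validating the old target, so only tagged parts of an object are affected.
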(fn StartHighlight
  (params (NewHighlight :type Actor%20Object%20Reference) (OldHighlight :type Actor%20Object%20Reference))
  (CallFunction|StopHighlight OldHighlight (LocalVariables|Get__WorldContext))
  (for _array_element (Actor|GetComponentsbyTag NewHighlight "/Script/Engine.PrimitiveComponent" "Highlight")
    (Rendering|SetRenderCustomDepth _array_element true)))

(fn StopHighlight
  (params (OldHighlight :type Actor%20Object%20Reference))
  (Utilities|IsValid OldHighlight
    (:Is%20Valid
      (if (not (== OldHighlight 0))
        (for _array_element (Actor|GetComponentsbyTag OldHighlight "/Script/Engine.PrimitiveComponent" "Highlight")
          (Rendering|SetRenderCustomDepth _array_element false))))))