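; A Blueprint function library of helpers that build forward-pointing segments from an actor or a component.
; Each returns a start vector at the world location and an end vector offset along the forward vector by a given distance or length.
; The start and end math lives in small sub-graphs, with separate versions for actors and components.
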(fn MForwardVector
  (params (Actor :type Actor%20Object%20Reference) (Distance :type Float%20%28single-precision%29))
  (bind _returnvalue (|StartVector Actor))
  ;[1 1 1] Given an actor and a distance, it returns the forward vector
  (return _returnvalue (|EndVector Actor _returnvalue Distance)))

(fn MForwardVectorComponent
  (params (Component :type Scene%20Component%20Object%20Reference) (Length :type Float%20%28single-precision%29))
  (bind _returnvalue (|StartVector Component))
  (return _returnvalue (|EndVector Component _returnvalue Length)))