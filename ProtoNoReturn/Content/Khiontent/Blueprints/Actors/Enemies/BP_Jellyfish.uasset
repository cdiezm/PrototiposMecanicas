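; Jellyfish enemy that drifts around its start location and damages the TPS player character on contact.
; Tick teleports it along independent cosine oscillations on X and Z, each set by a distance and speed.
; Sphere hits, gated by an attack cooldown, send OnAttackMessage and play the attack sound at the start location.
; An attached idle sound starts on BeginPlay and spawns again on each hit during cooldown.
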(event OnComponentHit(Sphere)
  (params (HitComponent :type Primitive%20Component%20Object%20Reference) (OtherActor :type Actor%20Object%20Reference) (OtherComp :type Primitive%20Component%20Object%20Reference) (NormalImpulse :type Vector :default "0, 0, 0") (Hit :type Hit%20Result%20Structure%20%28by%20ref%29))
  (if (>= (Variables|Default|GetAttackTime) (Variables|Default|GetKAttackTime))
    (Variables|Default|SetAttackTime 0.0)
    (Development|PrintString "Hello")
    (bind _asbp_tps_character (Utilities|Casting|CastToBP_TPS_Character OtherActor))
    (Class|IDamageable|OnAttack(Message) _asbp_tps_character (Variables|Default|GetDamage) "0, 0, 0")
    (Audio|PlaySoundatLocation "/Game/Khiontent/Sounds/Propios/Medusa/Medusa_Attack.Medusa_Attack" (Variables|Default|GetStartLocation))
    (else
      (Audio|SpawnSoundAttached "/Game/Khiontent/Sounds/Propios/Medusa/Medusa_Idle.Medusa_Idle" (Variables|Default|GetMesh) "None" "0, 0, 0" "0, 0, 0" "KeepRelativeOffset" true))))

(event EventBeginPlay
  (Transformation|SetActorLocation (Variables|Default|GetStartLocation) false false)
  (bind _returnvalue (Audio|SpawnSoundAttached "/Game/Khiontent/Sounds/Propios/Medusa/Medusa_Idle.Medusa_Idle" (Variables|Default|GetMesh) "None" "0, 0, 0" "0, 0, 0" "KeepRelativeOffset" true))
  (Variables|Default|SetIdle _returnvalue))

(event Collision|EventActorBeginOverlap
  (params (OtherActor :type Actor%20Object%20Reference)))

(event EventTick
  (params (DeltaSeconds :type Float%20%28single-precision%29))
  (Variables|Default|SetAttackTime (+ DeltaSeconds (Variables|Default|GetAttackTime)))
  (Variables|Default|SetSecondsAlive (+ DeltaSeconds (Variables|Default|GetSecondsAlive)))
  (Transformation|SetActorLocation (+ (Variables|Default|GetStartLocation) (Math|Vector|MakeVector (* (Variables|Default|GetMaxHorizontalDistance) (Math|Trig|Cos(Radians) (* (/ (Variables|Default|GetHorizontalMovementSpeed) (Variables|Default|GetMaxHorizontalDistance)) (Variables|Default|GetSecondsAlive)))) 0.0 (* (Variables|Default|GetMaxVerticalDistance) (Math|Trig|Cos(Radians) (* (/ (Variables|Default|GetVerticalMovementSpeed) (Variables|Default|GetMaxVerticalDistance)) (Variables|Default|GetSecondsAlive)))))) false true))

(fn ConstructionScript)