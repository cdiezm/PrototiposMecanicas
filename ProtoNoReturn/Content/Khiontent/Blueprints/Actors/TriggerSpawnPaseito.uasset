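; A one-shot trigger actor that spawns a Paseito AI character for Alpha Level 2 when an actor overlaps it.
; The first overlap sets a spawn flag, then spawns the configured character class at the spawn point actor's location.
; It stores references to the character and its AI controller, hands the controller the waypoint destination and calls its init event to start the behavior.
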(event Collision|EventActorBeginOverlap
  (params (OtherActor :type Actor%20Object%20Reference))
  (if (not (Variables|Default|GetHasSpawn))
    (Variables|Default|SetHasSpawn true)
    (bind _returnvalue (AI|SpawnAIFromClass (Variables|Default|GetIACharacter) 0 (Transformation|GetActorLocation (Variables|Default|GetSpawnPoint)) "0, 0, 0" false))
    (bind _asalpha_level_2_paseito (Utilities|Casting|CastToAlpha_Level2_Paseito _returnvalue))
    (bind _output_get (Variables|Default|SetIACharacterRef _asalpha_level_2_paseito))
    (bind _asiacontroller_alpha_level_2_paseito (Utilities|Casting|CastToIAControllerAlphaLevel2_Paseito (AI|GetAIController _output_get)))
    (bind _output_get_2 (Variables|Default|SetIAControllerRef _asiacontroller_alpha_level_2_paseito))
    (Variables|/Game/Khiontent/Blueprints/Classes/AIControllers/IAControllerAlphaLevel2_Paseito.IAControllerAlphaLevel2_Paseito_C|SetWaypointDestiny _output_get_2 (Variables|Default|GetWaypointDestiny))
    (Default|InitEvent _output_get_2)))

(fn ConstructionScript)