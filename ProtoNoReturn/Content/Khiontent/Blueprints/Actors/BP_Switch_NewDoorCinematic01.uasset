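; Trigger-based door switch that fires a camera cinematic once the player completes a button-mash QTE.
; Overlap shows the QTE widget, then either messages the doors immediately or, for use-required switches, enables input and fades the point light, with optional key gating.
; Each Use press taps the QTE; completion spawns a cinematic objective and long-hold camera trigger around the player, messages DoorsArray and sets the linked lights' switch-off probability.
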(event EventBeginPlay
  (|CallParentFunction) ; This node is disabled and will not be called.\nDrag off pins to build functionality.
)

(event Collision|EventActorBeginOverlap
  (params (OtherActor :type Actor%20Object%20Reference))
  (bind _bp_mashqte (Variables|Default|GetBP_MashQTE))
  (bind _asbp_tps_character (Utilities|Casting|CastToBP_TPS_Character OtherActor))
  (Variables|Default|SetCharacterReference _asbp_tps_character)
  (Variables|Default|SetIsInTrigger true)
  (Utilities|IsValid _bp_mashqte
    (:Is%20Valid
      (Default|ShowWidget _bp_mashqte))
    (:Is%20Not%20Valid
      _))
  (if (Variables|Default|GetNeedToUse)
    (if (Variables|Default|GetNeedKey)
      (if (Variables|/Game/Khiontent/Blueprints/Actors/BP_TPS_Character.BP_TPS_Character_C|GetHasKey (Variables|Default|GetCharacterReference))
        (Input|EnableInput (Game|GetPlayerController 0))
        (bind _alpha (Timeline|Timeline_5 PlayFromStart)
          (:Update
            (Rendering|Components|Light|SetIntensity (Variables|Default|GetPointLight) (Math|Float|Lerp (Variables|Default|GetLightMinimunIntensity) (Variables|Default|GetLightFullIntensity) _alpha))
            (Rendering|Components|Light|SetLightColor (Variables|Default|GetPointLight) (Variables|Default|GetIsInTriggerKeyNeededColor) true))
          (:Finished
            (Input|EnableInput (Game|GetPlayerController 0))))
        (else
          (Rendering|SetVisibility (Variables|Default|GetTexto) true false)
          (Timeline|Timeline_5 PlayFromStart)))
      (else
        (Input|EnableInput (Game|GetPlayerController 0))
        (bind _alpha_2 (Timeline|Timeline_4 Play)
          (:Update
            (Rendering|Components|Light|SetIntensity (Variables|Default|GetPointLight) (Math|Float|Lerp (Variables|Default|GetLightMinimunIntensity) (Variables|Default|GetLightFullIntensity) _alpha_2))
            (Rendering|Components|Light|SetLightColor (Variables|Default|GetPointLight) (Variables|Default|GetIsInTriggerBaseColor) true)))))
    (else
      (for _array_element (Variables|Default|GetDoors_Array)
        (if (Variables|Default|GetNeedKey)
          (if true
            (Class|UsableItemInterface|UseItem(Message) _array_element :!label _label))
          (else
            (goto _label)))))))

(event EventTick
  (params (DeltaSeconds :type Float%20%28single-precision%29)))

(event Input|ActionEvents|InputActionUse
  (params (Key :type Key%20Structure))
  (bind _returnvalue (Game|Player|GetPlayerPawn 0))
  (bind _returnvalue_2 (Transformation|GetActorTransform _returnvalue))
  (bind _location (Math|Transform|BreakTransform _returnvalue_2))
  (bind (_x _y _z) (Math|Vector|BreakVector _location))
  (:Pressed
    (if (Variables|Default|GetIsInTrigger)
      (if (Variables|Default|GetNeedKey)
        (if (Variables|/Game/Khiontent/Blueprints/Actors/BP_TPS_Character.BP_TPS_Character_C|GetHasKey (Variables|Default|GetCharacterReference))
          (Variables|Default|SetIsUSed true :!label _label)
          (Utilities|IsValid (Variables|Default|GetBP_MashQTE)
            (:Is%20Valid
              (Default|Tap (Variables|Default|GetBP_MashQTE))
              (bind _biscompleted (Default|IsQTECompleted (Variables|Default|GetBP_MashQTE)))
              (if _biscompleted
                (Default|DeleteWidget (Variables|Default|GetBP_MashQTE))
                (bind _returnvalue_3 (Game|SpawnActorfromClass "/Game/Gym/TestPedro/BP_CinematicObjective.BP_CinematicObjective_C" (Math|Transform|MakeTransform (Math|Vector|MakeVector (- _x 1e+03) _y (+ _z 5e+01))) "Undefined" 0 0))
                (bind _returnvalue_4 (Game|SpawnActorfromClass "/Game/Khiontent/Blueprints/Actors/BP_MoveCameraTrigger.BP_MoveCameraTrigger_C" (Math|Transform|MakeTransform (Math|Vector|MakeVector _x _y (+ _z 1e+02))) "Undefined" 0 0))
                (Variables|/Game/Khiontent/Blueprints/Actors/BP_MoveCameraTrigger.BP_MoveCameraTrigger_C|SetSecondsToKeepLookingAtObjective _returnvalue_4 99999.0)
                (Variables|/Game/Khiontent/Blueprints/Actors/BP_MoveCameraTrigger.BP_MoveCameraTrigger_C|SetPointToLookAt _returnvalue_4 _returnvalue_3)
                (for _array_element (Variables|Default|GetDoors_Array)
                  (Class|UsableItemInterface|UseItem(Message) _array_element))
                (for _array_element_2 (Variables|Default|GetLights)
                  (Variables|/Game/Khiontent/Blueprints/Actors/Luz.Luz_C|SetprobabilidadApagar _array_element_2 0.1)))))
          (else
            (Default|PrintMessage (Variables|Default|GetBP_PrintMessage))))
        (else
          (goto _label))))))

(fn ConstructionScript
  (|CallParentFunction))