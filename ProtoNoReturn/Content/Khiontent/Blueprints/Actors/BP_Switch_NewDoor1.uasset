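; Door switch actor that the player character works from its trigger area, optionally gated by holding a key.
; Overlap toggles player input and the mash QTE widget while timelines fade and recolor a point light; without NeedToUse, entry triggers the doors directly.
; Pressing Use taps the QTE.
; Completion sends UseItemMessage to linked doors, lowers ProbabilidadApagar on linked lights and removes the QTE.
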(event Custom|LlaveCogida
  (if (Variables|Default|GetNeedKey)
    _))

(event Collision|EventActorBeginOverlap
  (params (OtherActor :type Actor%20Object%20Reference))
  (bind _bp_mashqte (Variables|Default|GetBP_MashQTE))
  (bind _asbp_tps_character (Utilities|Casting|CastToBP_TPS_Character OtherActor))
  (Variables|Default|SetCharacterReference _asbp_tps_character)
  (Variables|Default|SetIsInTrigger true)
  (Utilities|IsValid _bp_mashqte
    (:Is%20Valid
      (Default|ShowWidget _bp_mashqte))
    (:Is%20Not%20Valid
      _))
  (if (Variables|Default|GetNeedToUse)
    (if (Variables|Default|GetNeedKey)
      (if (Variables|/Game/Khiontent/Blueprints/Actors/BP_TPS_Character.BP_TPS_Character_C|GetHasKey (Variables|Default|GetCharacterReference))
        (Input|EnableInput (Game|GetPlayerController 0))
        (bind _alpha (Timeline|Timeline_3 PlayFromStart)
          (:Update
            (Rendering|Components|Light|SetIntensity (Variables|Default|GetPointLight) (Math|Float|Lerp (Variables|Default|GetLightMinimunIntensity) (Variables|Default|GetLightFullIntensity) _alpha))
            (Rendering|Components|Light|SetLightColor (Variables|Default|GetPointLight) (Variables|Default|GetIsInTriggerKeyNeededColor) true))
          (:Finished
            (Input|EnableInput (Game|GetPlayerController 0))))
        (else
          (Rendering|SetVisibility (Variables|Default|GetTexto) true false)
          (Timeline|Timeline_3 PlayFromStart)))
      (else
        (Input|EnableInput (Game|GetPlayerController 0))
        (bind _alpha_2 (Timeline|Timeline_0 Play)
          (:Update
            (Rendering|Components|Light|SetIntensity (Variables|Default|GetPointLight) (Math|Float|Lerp (Variables|Default|GetLightMinimunIntensity) (Variables|Default|GetLightFullIntensity) _alpha_2))
            (Rendering|Components|Light|SetLightColor (Variables|Default|GetPointLight) (Variables|Default|GetIsInTriggerBaseColor) true)))))
    (else
      (for _array_element (Variables|Default|GetDoors_Array)
        (if (Variables|Default|GetNeedKey)
          (if true
            (Class|UsableItemInterface|UseItem(Message) _array_element :!label _label))
          (else
            (goto _label)))))))

(event EventDeleteHighlight
  (Utilities|IsValid (Variables|Default|GetMeshComponent)
    (:Is%20Valid
      (Components|DestroyComponent (Variables|Default|GetMeshComponent)))))

(event Collision|EventActorEndOverlap
  (params (OtherActor :type Actor%20Object%20Reference))
  (Utilities|Casting|CastToBP_TPS_Character OtherActor)
  (Variables|Default|SetIsInTrigger false)
  (if (Variables|Default|GetNeedKey)
    (Rendering|SetVisibility (Variables|Default|GetTexto) false false)
    (bind _alpha (Timeline|Timeline_2 ReverseFromEnd)
      (:Update
        (Rendering|Components|Light|SetIntensity (Variables|Default|GetPointLight) (Math|Float|Lerp (Variables|Default|GetLightMinimunIntensity) (Variables|Default|GetLightFullIntensity) _alpha))
        (Rendering|Components|Light|SetLightColor (Variables|Default|GetPointLight) (Variables|Default|GetKeyNeededColor) true)))
    (else
      (bind _alpha_2 (Timeline|Timeline_1 ReverseFromEnd)
        (:Update
          (Rendering|Components|Light|SetIntensity (Variables|Default|GetPointLight) (Math|Float|Lerp (Variables|Default|GetLightMinimunIntensity) (Variables|Default|GetLightFullIntensity) _alpha_2)))
        (:Finished
          (Rendering|Components|Light|SetLightColor (Variables|Default|GetPointLight) (Variables|Default|GetBaseColor) true)))))
  (Input|DisableInput (Game|GetPlayerController 0))
  (Utilities|IsValid (Variables|Default|GetBP_MashQTE)
    (:Is%20Valid
      (Default|HideWidget (Variables|Default|GetBP_MashQTE)))))

(event EventBeginPlay
  (if (Variables|Default|GetNeedKey)
    (Rendering|Components|Light|SetIntensity (Variables|Default|GetPointLight) (Variables|Default|GetLightMinimunIntensity))
    (Rendering|Components|Light|SetLightColor (Variables|Default|GetPointLight) (Variables|Default|GetKeyNeededColor) true)
    (else
      (Rendering|Components|Light|SetIntensity (Variables|Default|GetPointLight) (Variables|Default|GetLightMinimunIntensity))
      (Rendering|Components|Light|SetLightColor (Variables|Default|GetPointLight) (Variables|Default|GetBaseColor) true))))

(event EventSetComponentMesh
  (params (InMeshComponent :type Static%20Mesh%20Component%20Object%20Reference))
  (Variables|Default|SetMeshComponent InMeshComponent))

(event Input|ActionEvents|InputActionUse
  (params (Key :type Key%20Structure))
  (bind _bp_printmessage (Variables|Default|GetBP_PrintMessage))
  (:Pressed
    (if (Variables|Default|GetIsInTrigger)
      (if (Variables|Default|GetNeedKey)
        (if (Variables|/Game/Khiontent/Blueprints/Actors/BP_TPS_Character.BP_TPS_Character_C|GetHasKey (Variables|Default|GetCharacterReference))
          (Variables|Default|SetIsUSed true :!label _label)
          (Utilities|IsValid (Variables|Default|GetBP_MashQTE)
            (:Is%20Valid
              (Default|Tap (Variables|Default|GetBP_MashQTE))
              (bind _biscompleted (Default|IsQTECompleted (Variables|Default|GetBP_MashQTE)))
              (if _biscompleted
                (Default|StopPrintingMessage (Variables|Default|GetBP_PrintMessage))
                (Default|DeleteWidget (Variables|Default|GetBP_MashQTE))
                (for _array_element (Variables|Default|GetDoors_Array)
                  (Class|UsableItemInterface|UseItem(Message) _array_element))
                (for _array_element_2 (Variables|Default|GetLights)
                  (Variables|/Game/Khiontent/Blueprints/Actors/Luz.Luz_C|SetprobabilidadApagar _array_element_2 0.1))
                (Components|DestroyComponent (Variables|Default|GetBP_MashQTE))
                (else
                  (Variables|/Game/Khiontent/Blueprints/Classes/BP_PrintMessage.BP_PrintMessage_C|SetMessageText _bp_printmessage "Press repeatedly")
                  (Default|PrintMessage _bp_printmessage)))))
          (else
            (Default|PrintMessage (Variables|Default|GetBP_PrintMessage))))
        (else
          (goto _label))))))

(fn ConstructionScript)