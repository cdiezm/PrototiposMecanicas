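; Door actor that slides vertically between its initial position and a configurable open height, and can begin raised when set to open.
; UseItem drives a timeline forward or in reverse to lerp its Z, ignoring input mid-animation and flipping the open state on finish.
; CloseForever mutes the sound and zeroes the height after one move, so later uses leave it in place.
; Disconnected instant-move nodes remain unused.
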(event EventBeginPlay
  (Variables|Default|SetInitPos (Transformation|GetActorLocation))
  (if (Variables|Default|GetOpened)
    (Variables|Default|SetNextHeightToMove (* -1.0 (Variables|Default|GetHeightOpen)))
    (Transformation|SetActorLocation (Math|Vector|MakeVector (.x (Variables|Default|GetInitPos)) (.y (Variables|Default|GetInitPos)) (+ (.z (Variables|Default|GetInitPos)) (Variables|Default|GetHeightOpen))) false false)
    (else
      (Variables|Default|SetNextHeightToMove (Variables|Default|GetHeightOpen)))))

(event EventUseItem
  (bind _initpos (Variables|Default|GetInitPos))
  (bind _initpos_2 (Variables|Default|GetInitPos))
  (if (not (Variables|Default|GetIsInAnimation))
    (if (Variables|Default|GetCloseForever)
      _
      (else
        (Audio|PlaySound2D "/Game/Khiontent/Sounds/Close_door_sound.Close_door_sound")))
    (Variables|Default|SetIsInAnimation true)
    (if (Variables|Default|GetOpened)
      (bind _alpha (Timeline|Timeline_0 ReverseFromEnd)
        (:Update
          (Transformation|SetActorLocation (Math|Vector|MakeVector (.x _initpos_2) (.y _initpos_2) (Math|Float|Lerp (.z _initpos) (+ (.z _initpos) (Variables|Default|GetHeightOpen)) _alpha)) false false))
        (:Finished
          (Variables|Default|SetIsInAnimation false)
          (Variables|Default|SetOpened (not (Variables|Default|GetOpened)))
          (if (Variables|Default|GetCloseForever)
            (Variables|Default|SetHeightOpen 0.0))))
      (else
        (Timeline|Timeline_0 PlayFromStart)))))

(fn ConstructionScript)