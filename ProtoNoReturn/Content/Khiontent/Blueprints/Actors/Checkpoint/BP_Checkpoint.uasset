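; Checkpoint actor that auto-saves the game when the TPS character overlaps it, with a trigger box resizable through the construction script.
; A DoOnce lets it fire once, and it saves only while the GameInstance's SavedGame flag is false, then sets that flag.
; It writes health, temperature, bracelet energy and location into a new BP_SavedValues object in slot Save_001, clears the new-level flag and prints a confirmation.
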(event Collision|EventActorBeginOverlap
  (params (OtherActor :type Actor%20Object%20Reference))
  (bind _asbp_tps_character (Utilities|Casting|CastToBP_TPS_Character OtherActor))
  (Variables|Default|SetCharacter _asbp_tps_character)
  (bind _returnvalue (SaveGame|CreateSaveGameObject "/Game/Khiontent/Blueprints/Actors/Checkpoint/BP_SavedValues.BP_SavedValues_C"))
  (Variables|Default|SetSave _returnvalue)
  (Utilities|FlowControl|DoOnce false
    (:Completed
      (bind _asgame_instance_to_level_muerte (Utilities|Casting|CastToGameInstanceToLevelMuerte (Game|GetGameInstance)))
      (if (not (Variables|/Game/Khiontent/Blueprints/GameInstances/GameInstanceToLevelMuerte.GameInstanceToLevelMuerte_C|GetSavedGame _asgame_instance_to_level_muerte))
        (Variables|/Game/Khiontent/Blueprints/Actors/Checkpoint/BP_SavedValues.BP_SavedValues_C|SetHealth (Variables|Default|GetSave) (Variables|/Game/Khiontent/Blueprints/Actors/BP_TPS_Character.BP_TPS_Character_C|GetcurrentHP (Variables|Default|GetCharacter)))
        (Variables|/Game/Khiontent/Blueprints/Actors/Checkpoint/BP_SavedValues.BP_SavedValues_C|SetTemperature (Variables|Default|GetSave) (Variables|/Game/Khiontent/Blueprints/Classes/Temperature_Comp.Temperature_Comp_C|GetTemperature (Variables|/Game/Khiontent/Blueprints/Actors/BP_TPS_Character.BP_TPS_Character_C|GetTemperature_Comp (Variables|Default|GetCharacter))))
        (bind _currentenergy (Default|GetCurrentEnergy (Variables|/Game/Khiontent/Blueprints/Actors/BP_TPS_Character.BP_TPS_Character_C|GetBP_Bracelet (Variables|Default|GetCharacter))))
        (Variables|/Game/Khiontent/Blueprints/Actors/Checkpoint/BP_SavedValues.BP_SavedValues_C|SetEnergy (Variables|Default|GetSave) _currentenergy)
        (Variables|/Game/Khiontent/Blueprints/Actors/Checkpoint/BP_SavedValues.BP_SavedValues_C|SetLocation (Variables|Default|GetSave) (Transformation|GetActorLocation (Variables|Default|GetCharacter)))
        (Variables|/Game/Khiontent/Blueprints/Actors/Checkpoint/BP_SavedValues.BP_SavedValues_C|SetblsNewLevel (Variables|Default|GetSave) false)
        (SaveGame|SaveGametoSlot (Variables|Default|GetSave) "Save_001")
        (bind _asgame_instance_to_level_muerte_2 (Utilities|Casting|CastToGameInstanceToLevelMuerte (Game|GetGameInstance)))
        (Variables|/Game/Khiontent/Blueprints/GameInstances/GameInstanceToLevelMuerte.GameInstanceToLevelMuerte_C|SetSavedGame _asgame_instance_to_level_muerte_2 true)
        (Development|PrintString "Game Saved")))))

(fn ConstructionScript
  (Components|Box|SetBoxExtent (Variables|Default|GetTrigger) (Variables|Default|GetTriggerResize) true))