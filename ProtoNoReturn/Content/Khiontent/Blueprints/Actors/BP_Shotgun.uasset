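; Shotgun actor attached to BP_TPS_Character that shows a laser sight with an impact decal while the player aims.
; Each tick it line-traces from the follow camera with a lerped end point, or along the laser component during the ironsights fire montage.
; The beam component is destroyed and re-created at each update to run from the laser to the target.
; When not aiming, it clears the beams and hides the decal.
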(event EventTick
  (params (DeltaSeconds :type Float%20%28single-precision%29))
  (bind _beamarray (Variables|Default|GetBeamArray))
  (if (Variables|Default|GetPlayerIsAiming)
    (bind _asbp_tps_character (Utilities|Casting|CastToBP_TPS_Character (Actor|GetAttachParentActor)))
    (bind _returnvalue (Animation|GetCurrentMontage _asbp_tps_character :!class /Script/Engine.Character))
    (if (== _returnvalue "/Game/Khiontent/Animations/Animations_Proto_Stealth/Final/Fire_Shotgun_Ironsights_Montage.Fire_Shotgun_Ironsights_Montage")
      (bind (_start_vector _end_vector) (CallFunction|MForwardVectorComponent (Variables|Default|GetLaserBeam) 5e+03))
      (bind _end (|CollapseGraph_0_3 _start_vector _end_vector _start_vector))
      (else
        (bind (_start_vector_2 _end_vector_2) (CallFunction|MForwardVectorComponent (Variables|/Game/Khiontent/Blueprints/Actors/BP_TPS_Character.BP_TPS_Character_C|GetFollowCamera _asbp_tps_character) 5e+03))
        (Variables|Default|SetAlpha (Math|Float|Clamp(Float) (Variables|Default|GetAlpha) 0.0))
        (|CollapseGraph_0 _start_vector_2 (Math|Vector|Lerp(Vector) _end _end_vector_2 (+ (Variables|Default|GetAlpha) 0.4)) (Transformation|GetWorldLocation (Variables|Default|GetLaserBeam)))))
    (else
      (Class|ParticleSystemComponent|SetBeamSourcePoint (Variables|Default|GetLaserBeam) 0 "0, 0, 0")
      (Class|ParticleSystemComponent|SetBeamTargetPoint (Variables|Default|GetLaserBeam) 0 "0, 0, 0")
      (Rendering|SetVisibility (Variables|Default|GetLaserDecal) false false)
      (for _array_element _beamarray
        (Utilities|IsValid _array_element
          (:Is%20Valid
            (Components|DestroyComponent _array_element))))
      (Utilities|Array|Clear _beamarray))))

(fn ConstructionScript
  (Collision|SetCollisionResponsetoAllChannels (Variables|Default|GetShotgun) "ECR_Ignore"))

(fn Laser
  (Effects|Components|ParticleSystem|SetTemplate (Variables|Default|GetLaserBeam) "/Game/Khiontent/Particles/LaserPS.LaserPS"))

(fn AddNewBeam
  (params (Start :type Vector) (End :type Vector))
  (bind _returnvalue (AddComponent|AddParticleSystemComponent false))
  (Utilities|Array|Add (Variables|Default|GetBeamArray) _returnvalue)
  (Class|ParticleSystemComponent|SetBeamSourcePoint _returnvalue 0 Start)
  (Class|ParticleSystemComponent|SetBeamTargetPoint _returnvalue 0 End))