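; Trigger actor that recharges a player's bracelet while the character stands inside it.
; On begin overlap it takes the bracelet from a TPS or Conduit character and tells its BPRechargeBracelet to start recharging it.
; On end overlap it resolves the bracelet the same way and stops the recharge.
; Both events ignore other actors and only act on a valid bracelet.
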(event Collision|EventActorBeginOverlap
  (params (OtherActor :type Actor%20Object%20Reference))
  (bind _asbp_tps_character (Utilities|Casting|CastToBP_TPS_Character OtherActor)
    (:then
      (Variables|Default|SetBraceletToRecharge (Variables|/Game/Khiontent/Blueprints/Actors/BP_TPS_Character.BP_TPS_Character_C|GetBP_Bracelet _asbp_tps_character)))
    (:CastFailed
      (bind _asbp_character_conduit (Utilities|Casting|CastToBP_Character_Conduit OtherActor))
      (Variables|Default|SetBraceletToRecharge (Variables|/Game/Khiontent/Blueprints/Actors/BP_Character_Conduit.BP_Character_Conduit_C|GetBP_Bracelet _asbp_character_conduit))))
  (Utilities|IsValid (Variables|Default|GetBraceletToRecharge)
    (:Is%20Valid
      (Default|RechargeBracelet (Variables|Default|GetBP_RechargeBracelet) (Variables|Default|GetBraceletToRecharge)))))

(event Collision|EventActorEndOverlap
  (params (OtherActor :type Actor%20Object%20Reference))
  (bind _asbp_tps_character (Utilities|Casting|CastToBP_TPS_Character OtherActor)
    (:then
      (Variables|Default|SetBraceletToRecharge (Variables|/Game/Khiontent/Blueprints/Actors/BP_TPS_Character.BP_TPS_Character_C|GetBP_Bracelet _asbp_tps_character)))
    (:CastFailed
      (bind _asbp_character_conduit (Utilities|Casting|CastToBP_Character_Conduit OtherActor))
      (Variables|Default|SetBraceletToRecharge (Variables|/Game/Khiontent/Blueprints/Actors/BP_Character_Conduit.BP_Character_Conduit_C|GetBP_Bracelet _asbp_character_conduit))))
  (Utilities|IsValid (Variables|Default|GetBraceletToRecharge)
    (:Is%20Valid
      (Default|StopRechargingBracelet (Variables|Default|GetBP_RechargeBracelet) (Variables|Default|GetBraceletToRecharge)))))

(fn ConstructionScript)