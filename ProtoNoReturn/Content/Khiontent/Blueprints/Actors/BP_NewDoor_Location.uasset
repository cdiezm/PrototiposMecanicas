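; Sliding door actor that moves between its placed location and a target offset along world Y by a configurable distance.
; BeginPlay caches both positions and snaps the door to the target when it starts open.
; OpenDoor toggles IsOpened and plays or reverses a timeline at a set rate, lerping the location with its alpha track.
; The timeline clears IsInAnim when it finishes.
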(event EventBeginPlay
  (bind _output_get (Variables|Default|SetActualLocation (Transformation|GetActorLocation)))
  (Variables|Default|SetTargetLocation (Math|Vector|MakeVector (.x _output_get) (+ (.y _output_get) (Variables|Default|GetCentimetresToMove%20%28ToRight%29)) (.z _output_get)))
  (if (Variables|Default|GetIsOpened)
    (Transformation|SetActorLocation (Variables|Default|GetTargetLocation) false false)))

(event EventOpenDoor
  (params (Is%20Opened :type Boolean))
  (Components|Timeline|SetPlayRate (Variables|Default|GetOpen%20Door%20Timeline) (Variables|Default|GetPlayRate))
  (if Is%20Opened
    (Variables|Default|SetIsOpened (not (Variables|Default|GetIsOpened)))
    (bind _rotation_alpha (Timeline|Open%20Door%20Timeline Reverse)
      (:Update
        (Transformation|SetActorLocation (Math|Vector|Lerp(Vector) (Variables|Default|GetActualLocation) (Variables|Default|GetTargetLocation) _rotation_alpha) false false))
      (:Finished
        (Variables|Default|SetIsInAnim false)))
    (else
      (Variables|Default|SetIsOpened (not (Variables|Default|GetIsOpened)))
      (Timeline|Open%20Door%20Timeline Play))))

(fn ConstructionScript)