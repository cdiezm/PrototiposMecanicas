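; Rotating door actor that swings between closed and open yaw angles.
; BeginPlay caches the starting rotation, derives the target from a clockwise degree offset, and snaps to it if the door starts opened.
; OpenDoor flips IsOpened and plays or reverses a timeline at PlayRate, whose alpha lerps the actor rotation between the two.
; The timeline clears IsInAnim when it finishes.
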(event EventBeginPlay
  (bind _output_get (Variables|Default|SetActualRotation (Transformation|GetActorRotation)))
  (Variables|Default|SetTargetRotation (Math|Rotator|MakeRotator (.roll _output_get) (.pitch _output_get) (+ (.yaw _output_get) (Variables|Default|GetDegreesToRotClockwise))))
  (if (Variables|Default|GetIsOpened)
    (Transformation|SetActorRotation (Variables|Default|GetTargetRotation))))

(event EventOpenDoor
  (params (Is%20Opened :type Boolean))
  (Components|Timeline|SetPlayRate (Variables|Default|GetOpen%20Door%20Timeline) (Variables|Default|GetPlayRate))
  (if Is%20Opened
    (Variables|Default|SetIsOpened (not (Variables|Default|GetIsOpened)))
    (bind _rotation_alpha (Timeline|Open%20Door%20Timeline Reverse)
      (:Update
        (Transformation|SetActorRotation (Math|Rotator|Lerp(Rotator) (Variables|Default|GetActualRotation) (Variables|Default|GetTargetRotation) _rotation_alpha)))
      (:Finished
        (Variables|Default|SetIsInAnim false)))
    (else
      (Variables|Default|SetIsOpened (not (Variables|Default|GetIsOpened)))
      (Timeline|Open%20Door%20Timeline Play))))

(fn ConstructionScript)