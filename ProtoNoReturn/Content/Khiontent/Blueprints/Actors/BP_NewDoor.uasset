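; Base door Blueprint that handles being used and leaves the actual opening to child Blueprints.
; UseItem ignores repeat uses when OnlyOneUse is set, otherwise it flags the door as used and animating, then calls OpenDoor with IsOpened.
; The 2D sound plays only when no animation is flagged, and IsInAnim is never cleared here.
; OpenDoor is intentionally empty so children can implement it.
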(event Custom|Open%20Door
  (params (Is%20Opened :type Boolean)))

(event EventUseItem
  (if (Variables|Default|GetOnlyOneUse)
    (if (not (Variables|Default|GetIsUsed))
      (if (Variables|Default|GetIsInAnim) :!label _label
        _
        (else
          (Audio|PlaySound2D (Variables|Default|GetSound))))
      (Variables|Default|SetIsInAnim true)
      (Variables|Default|SetIsUsed true)
      (CallFunction|OpenDoor (Variables|Default|GetIsOpened)))
    (else
      (goto _label))))

(fn ConstructionScript)