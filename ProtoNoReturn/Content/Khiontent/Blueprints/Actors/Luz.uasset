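; Luz is a light actor that flickers at random.
; On BeginPlay it stores the light's starting intensity and starts a looping timer at the VelocidadParpadeo interval.
; Each timer call to Parpadear rolls a random float against ProbabilidadApagar, setting the intensity to zero or restoring the stored value.
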(event EventBeginPlay
  (Variables|Default|SetintensidadInicial (Variables|/Script/Engine.LightComponentBase|GetIntensity (Variables|Default|GetLuz)))
  (Utilities|Time|SetTimerbyFunctionName 0 "parpadear" (Variables|Default|GetvelocidadParpadeo) true))

(event Collision|EventActorBeginOverlap
  (params (OtherActor :type Actor%20Object%20Reference)))

(event EventTick
  (params (DeltaSeconds :type Float%20%28single-precision%29)))

(fn ConstructionScript)

(fn Parpadear
  (if (>= (Variables|Default|GetprobabilidadApagar) (Math|Random|RandomFloat))
    (Rendering|Components|Light|SetIntensity (Variables|Default|GetLuz) 0.0)
    (else
      (Rendering|Components|Light|SetIntensity (Variables|Default|GetLuz) (Variables|Default|GetintensidadInicial)))))