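; Alpha is a ghost-themed enemy pawn that chases the player on sight and damages them when close.
; Pawn sensing triggers a one-time alert sound and AI MoveTo, then sends an attack message if the character's proximity check passes.
; Incoming attacks play size-dependent sounds, spawn optional ice/blood effects and reduce HP until destruction.
; A hit halts movement and sets IsHitted, never cleared here, blocking further chasing.
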(event OnSeePawn(PawnSensing)
  (params (Pawn :type Pawn%20Object%20Reference))
  ;[1 1 1] Perseguir
  (if (not (Variables|Default|GetIs%20Hitted))
    (bind _asbp_tps_character (Utilities|Casting|CastToBP_TPS_Character Pawn))
    (Variables|Default|SetPersonaje _asbp_tps_character)
    (if (Variables|Default|GetMeHaVisto)
      _
      (else
        (Audio|PlaySoundatLocation "/Game/Khiontent/Sounds/13__Ghost1.13__Ghost1" (Transformation|GetActorLocation))
        (Variables|Default|SetMeHaVisto true)))
    (AI|AIMoveTo self "0, 0, 0" _asbp_tps_character 5.0 false
      (:OnSuccess
        (if (|SiElPersonajeEstaCerca _asbp_tps_character)
          (Class|IDamageable|OnAttack(Message) _asbp_tps_character (Variables|Default|GetDamage) "0, 0, 0"))))))

(event EventOnAttack
  (params (Damage :type Float%20%28single-precision%29) (Location :type Vector :default "0, 0, 0"))
  (bind _returnvalue (Transformation|GetActorLocation))
  (bind _self self)
  (bind _particlesscale (Variables|Default|GetParticlesScale))
  (bind _returnvalue_2 (Transformation|GetActorTransform _self))
  (if (Variables|Default|GetIsCanijo)
    (Audio|PlaySoundatLocation "/Game/Khiontent/Sounds/Impacto_Peque.Impacto_Peque" _returnvalue "0, 0, 0" 0.5 0.4 1.0)
    (else
      (Audio|PlaySoundatLocation "/Game/Khiontent/Sounds/Ice_Impact.Ice_Impact" _returnvalue "0, 0, 0" 0.5 0.4 1.0)))
  (Variables|Default|SetIs%20Hitted true)
  (if (Variables|Default|GetParticlesWhenDamaged)
    (Game|SpawnActorfromClass "/Game/Khiontent/Blueprints/Actors/BP_Ice_Impact.BP_Ice_Impact_C" (Math|Transform|MakeTransform Location "0, 0, 0" (Math|Vector|MakeVector _particlesscale _particlesscale _particlesscale)) "AlwaysSpawn" 0 0))
  (if (Variables|Default|GetBloodWhenDamaged)
    (Game|SpawnActorfromClass "/Game/Khiontent/Blueprints/Actors/Mancha_Sangre_Enemigo.Mancha_Sangre_Enemigo_C" (Math|Transform|MakeTransform (Math|Vector|MakeVector (.x (.location _returnvalue_2)) (.y (.location _returnvalue_2)) 0.0) (.rotation _returnvalue_2) (.scale _returnvalue_2)) "AlwaysSpawn" 0 0))
  (bind _output_get (Variables|Default|SetHP (- (Variables|Default|GetHP) Damage)))
  (if (<= _output_get 0.0)
    (Audio|PlaySound2D "/Game/Khiontent/Sounds/breathe_ghost_eerie.breathe_ghost_eerie" 0.5)
    (Actor|DestroyActor)
    (else
      (Components|Movement|StopMovementImmediately (Variables|Character|GetCharacterMovement))
      (if (not (Variables|Default|GetIs%20Hitted))
        (AI|AIMoveTo self "0, 0, 0" (Variables|Default|GetPersonaje) 5.0 false)))))

(fn ConstructionScript
  ;[1 1 1] Velocidad del enemigo
  (Variables|/Script/Engine.CharacterMovementComponent|SetMaxWalkSpeed (Variables|Character|GetCharacterMovement) (Variables|Default|GetSpeed)))