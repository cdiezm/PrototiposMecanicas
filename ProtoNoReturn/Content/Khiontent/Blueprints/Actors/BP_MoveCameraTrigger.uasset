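; Trigger actor that plays a short camera cinematic when a TPS or Conduit character overlaps it, showing a point of interest.
; It disables input, moves the character's follow camera to a target point facing a look-at point (both default to itself), holds with a sound cue, then reverses.
; Two timelines with duration-derived play rates drive the blend and hold.
; Input returns afterward, and the trigger optionally destroys itself for one-time use.
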(event Collision|EventActorBeginOverlap
  (params (OtherActor :type Actor%20Object%20Reference))
  (if (!= (Variables|Default|GetPointToMoveCameraTo) 0)
    _
    (else
      (Variables|Default|SetPointToMoveCameraTo self)))
  (if (!= (Variables|Default|GetPointToLookAt) 0)
    _
    (else
      (Variables|Default|SetPointToLookAt self)))
  (bind _asbp_tps_character (Utilities|Casting|CastToBP_TPS_Character OtherActor)
    (:then
      (Variables|Default|SetCurrentOverlappedActor _asbp_tps_character)
      (Variables|Default|SetCurrentOverlappedComponent (Variables|/Game/Khiontent/Blueprints/Actors/BP_TPS_Character.BP_TPS_Character_C|GetFollowCamera _asbp_tps_character))
      (Variables|Default|SetCurrentOverlappedCamera (Variables|/Game/Khiontent/Blueprints/Actors/BP_TPS_Character.BP_TPS_Character_C|GetFollowCamera _asbp_tps_character)))
    (:CastFailed
      (bind _asbp_character_conduit (Utilities|Casting|CastToBP_Character_Conduit OtherActor))
      (Variables|Default|SetCurrentOverlappedActor _asbp_character_conduit)
      (Variables|Default|SetCurrentOverlappedComponent (Variables|/Game/Khiontent/Blueprints/Actors/BP_Character_Conduit.BP_Character_Conduit_C|GetFollowCamera _asbp_character_conduit))
      (Variables|Default|SetCurrentOverlappedCamera (Variables|/Game/Khiontent/Blueprints/Actors/BP_Character_Conduit.BP_Character_Conduit_C|GetFollowCamera _asbp_character_conduit))))
  (Input|DisableInput (Variables|Default|GetCurrentOverlappedActor) 0)
  (Variables|Default|SetTemporaryVector (Transformation|GetWorldLocation (Variables|Default|GetCurrentOverlappedComponent)))
  (Variables|Default|SetTemporaryRotator (Transformation|GetWorldRotation (Variables|Default|GetCurrentOverlappedComponent)))
  (|SetPlayRates)
  (|PlayCinematic (Variables|Default|GetCurrentOverlappedCamera) (Math|Rotator|FindLookatRotation (Transformation|GetWorldLocation (Variables|Default|GetCurrentOverlappedCamera)) (Transformation|GetWorldLocation (Variables|/Script/Engine.Actor|GetRootComponent (Variables|Default|GetPointToLookAt)))) (Variables|Default|GetTemporaryVector) (Transformation|GetActorLocation (Variables|Default|GetPointToMoveCameraTo)))
  (Input|EnableInput (Variables|Default|GetCurrentOverlappedActor) 0)
  (if (Variables|Default|GetbIsActivatedFirstTimeOnly)
    (Actor|DestroyActor)))

(fn ConstructionScript)