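; BP_Conduit is a trigger actor that moves the player between the third-person character and the conduit character.
; Overlap with either pawn records the direction, enables input and shows the matching enter or exit prompt until the overlap ends.
; On Use, it spawns the other pawn at a preset point, lerps the current camera to the new view on a Timeline, then possesses the new pawn and destroys the old one.
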(event EventBeginPlay)

(event Collision|EventActorBeginOverlap
  (params (OtherActor :type Actor%20Object%20Reference))
  (bind _asbp_tps_character (Utilities|Casting|CastToBP_TPS_Character OtherActor)
    (:then
      (Variables|Default|SetCharacterOut _asbp_tps_character)
      (Variables|Default|SetIsEntering true))
    (:CastFailed
      (bind _asbp_character_conduit (Utilities|Casting|CastToBP_Character_Conduit OtherActor))
      (Variables|Default|SetCharacterIn _asbp_character_conduit)
      (Variables|Default|SetIsEntering false)))
  (Variables|Default|SetIsInTrigger true)
  (Input|EnableInput (Game|GetPlayerController 0))
  (if (Variables|Default|GetIsEntering)
    (Rendering|SetVisibility (Variables|Default|GetUseTextEntering) true false)
    (else
      (Rendering|SetVisibility (Variables|Default|GetUseTextExiting) true false))))

(event EventTick
  (params (DeltaSeconds :type Float%20%28single-precision%29)))

(event Collision|EventActorEndOverlap
  (params (OtherActor :type Actor%20Object%20Reference))
  (Utilities|Casting|CastToBP_TPS_Character OtherActor
    (:then
      _)
    (:CastFailed
      (Utilities|Casting|CastToBP_Character_Conduit OtherActor)))
  (Variables|Default|SetIsInTrigger false)
  (Input|DisableInput (Game|GetPlayerController 0))
  (Rendering|SetVisibility (Variables|Default|GetUseTextEntering) false false)
  (Rendering|SetVisibility (Variables|Default|GetUseTextExiting) false false))

(event Input|ActionEvents|InputActionUse
  (params (Key :type Key%20Structure))
  (:Pressed
    (if (Variables|Default|GetIsInTrigger)
      (if (Variables|Default|GetIsEntering)
        (|EntertoConduit)
        (else
          (|ExitConduit))))))

(fn ConstructionScript)