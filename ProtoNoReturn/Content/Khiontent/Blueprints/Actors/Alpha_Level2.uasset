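; Alpha enemy actor for Level 2 that exposes attack and audio events for patrolling and hitting a conduit.
; BeginPlay caches the first BP_TPS_Character and starts patrol and freeze audio, while Tick keeps the conduit-death viewpoint location updated.
; AttackPlayer deals massive damage through the player's OnAttack, re-finding the character if the reference is invalid.
; Other events fade patrol audio or play randomized, pitch-varied hit sounds, never picking the last array entry.
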(event Custom|AttackPlayer
  (Utilities|IsValid (Variables|Default|GetPlayerRef)
    (:Is%20Valid
      (Default|OnAttack (Variables|Default|GetPlayerRef) 2e+03 "0, 0, 0" :!label _label))
    (:Is%20Not%20Valid
      (bind _outactors (Actor|GetAllActorsOfClass "/Game/Khiontent/Blueprints/Actors/BP_TPS_Character.BP_TPS_Character_C"))
      (bind _output_get (Variables|Default|SetPlayerRef (Utilities|Array|Get(acopy) _outactors)))
      (Utilities|IsValid _output_get
        (:Is%20Valid
          (goto _label))
        (:Is%20Not%20Valid
          (Development|PrintString "NO CHARACTER FOUND!" true true "(R=1.000000,G=0.036710,B=0.000000,A=1.000000)" 1e+01))))))

(event Custom|StopPatrolSound
  (Audio|Components|Audio|FadeOut (Variables|Default|GetAudioPatrol) 1.0 0.0 :!class /Script/Engine.AudioComponent))

(event Custom|PlayPatrolSound
  (Audio|Components|Audio|FadeIn (Variables|Default|GetAudioPatrol) 1.0 1.0 0.0 :!class /Script/Engine.AudioComponent))

(event Custom|PlaySoundHitConduit
  (bind _hitsounds (Variables|Default|GetHitSounds))
  (bind _audiohitconduit (Variables|Default|GetAudioHitConduit))
  (Audio|Components|Audio|SetSound (Variables|Default|GetAudioHitConduit) (Utilities|Array|Get(acopy) _hitsounds (Math|Random|RandomInteger (- (Utilities|Array|Length _hitsounds) 1))))
  (Audio|Components|Audio|SetPitchMultiplier _audiohitconduit (Math|Random|RandomFloatinRange 0.8 1.0))
  (Audio|Components|Audio|Play _audiohitconduit 0.0))

(event EventBeginPlay
  (Variables|Default|SetIsHittingConduit false)
  (Variables|Default|SetPointOfViewConduitDeathLocation (Transformation|GetWorldLocation (Variables|Default|GetPointToViewConduitDeath)))
  (bind _outactors (Actor|GetAllActorsOfClass "/Game/Khiontent/Blueprints/Actors/BP_TPS_Character.BP_TPS_Character_C"))
  (Variables|Default|SetPlayerRef (Utilities|Array|Get(acopy) _outactors))
  (Audio|Components|Audio|Play (Variables|Default|GetAudioPatrol) 0.0)
  (Audio|Components|Audio|Play (Variables|Default|GetAudioFreeze) 0.0))

(event EventTick
  (params (DeltaSeconds :type Float%20%28single-precision%29))
  ;[1 1 1] Se que es una cerdada, pero ahora mismo no me da la cabeza para mas
  (Variables|Default|SetPointOfViewConduitDeathLocation (Transformation|GetWorldLocation (Variables|Default|GetPointToViewConduitDeath))))

(fn ConstructionScript)